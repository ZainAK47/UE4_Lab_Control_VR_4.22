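; Free-camera character that stands in for the VR motion controller pawn when no headset is connected.
; CheckHMDAndSwitchIfNone activates camera and movement, possesses this character, attaches the pawn's right controller at an offset and hides the left.
; Input axes drive look and movement, with a jump action and a hold-to-zoom timeline that slides the camera along X.
; A push action animates the right controller forward by timeline and resets it on release.
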(event `self.ReceiveBeginPlay`)

(event `InputAxis|FreeCameraTurn`
  (params (AxisValue :type "Float (single-precision)"))
  (`self.AddControllerYawInput` AxisValue))

(event `InputAxis|FreeCameraLookUp`
  (params (AxisValue :type "Float (single-precision)"))
  (`self.AddControllerPitchInput` (* AxisValue -1.0)))

(event `InputAxis|FreeCameraMoveForward`
  (params (AxisValue :type "Float (single-precision)"))
  (`self.AddMovementInput` (`self.GetActorForwardVector`) AxisValue))

(event `InputAxis|FreeCameraMoveRight`
  (params (AxisValue :type "Float (single-precision)"))
  (`self.AddMovementInput` (`self.GetActorRightVector`) AxisValue))

(event `InputAction|FreeCameraZoom`
  (params (Key :type "Key Structure"))
  (:`Pressed`
    (bind (_direction _zoomtrack) (`Timeline|ZoomCamera` :!via `PlayFromStart` :!label _label)
      (:`Update`
        (`SceneComponent.K2_SetRelativeLocation` (`self.Camera`) (`KismetMathLibrary.MakeVector` _zoomtrack) false false))))
  (:`Released`
    (goto _label :!via `ReverseFromEnd`)))

(event `InputAction|FreeCameraJump`
  (params (Key :type "Key Structure"))
  (:`Pressed`
    (`self.Jump`)))

(event `InputAction|FreeCameraPushRightControllerForward` :consume false
  (params (Key :type "Key Structure"))
  (bind _nonvrcontrollerdisplacement (`self.NonVRControllerDisplacement`))
  (bind _rightcontroller (`/Game/VirtualRealityBP/Blueprints/MotionControllerPawn.RightController` (`self.MotionControllerPawnRef`)))
  (:`Pressed`
    (bind (_direction _pushx) (`Timeline|PushProfile` :!via `PlayFromStart`)
      (:`Update`
        (`self.K2_SetActorRelativeLocation` _rightcontroller (`KismetMathLibrary.MakeVector` (+ _pushx (.x _nonvrcontrollerdisplacement)) (.y _nonvrcontrollerdisplacement) (.z _nonvrcontrollerdisplacement)) false false))))
  (:`Released`
    (`self.K2_SetActorRelativeLocation` _rightcontroller _nonvrcontrollerdisplacement false false)))

(fn `CheckHMDAndSwitchIfNone`
  (params (MotionControllerPawnReference :type "/Game/VirtualRealityBP/Blueprints/MotionControllerPawn Object Reference"))
  (bind _rightcontroller (`/Game/VirtualRealityBP/Blueprints/MotionControllerPawn.RightController` MotionControllerPawnReference))
  (set `self.MotionControllerPawnRef` MotionControllerPawnReference)
  (if (not (`HeadMountedDisplayFunctionLibrary.IsHeadMountedDisplayConnected`))
    (`ActorComponent.SetActive` (`self.Camera`) true false)
    (`ActorComponent.SetActive` (`self.CharacterMovement`) true false)
    (`Controller.Possess` (`GameplayStatics.GetPlayerController` 0) self)
    (`self.K2_AttachToActor` _rightcontroller self "None" "SnapToTarget" "SnapToTarget" "KeepRelative" true)
    (`self.K2_SetActorRelativeLocation` _rightcontroller (`self.NonVRControllerDisplacement`) false false)
    (`self.SetActorHiddenInGame` (`/Game/VirtualRealityBP/Blueprints/MotionControllerPawn.LeftController` MotionControllerPawnReference) true)))

(fn `UserConstructionScript`)