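; Receiver Blueprint that feeds incoming data, presumably UDP as the name suggests, to a 3D crane implementation.
; Each Tick polls for new data and delivers its five floats to the crane reference as X, Y, Z, Alpha and Beta.
; Separately, BeginPlay starts a Timeline that sends synthetic position and angle values, without Z, to two FakeData targets, apparently for testing.
; A FlipFlop on Finished ping-pongs that Timeline indefinitely.
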(event `self.ReceiveTick`
  (params (DeltaSeconds :type "Float (single-precision)"))
  (bind _returnvalue (`self.IsNewDataReady`))
  (if _returnvalue
    (bind _returnvalue_2 (`self.GetData`))
    (bind (_float1 _float2 _float3 _float4 _float5) (break `UDPData` _returnvalue_2))
    (message `/Game/Blueprints/3DCraneDDeliverInterface.DeliverData` (`self.3DCraneImplRef`) _float1 _float2 _float3 _float4 _float5)))

(event `self.ReceiveBeginPlay`
  ;[1 1 1] Probably made for some kind of test
  (bind (_direction _x _a) (`Timeline|Timeline_0` :!label _label)
    (:`Update`
      (message `/Game/Blueprints/3DCraneDDeliverInterface.DeliverData` (`self.FakeData`) _x _x 0.0 _a _a)
      (message `/Game/Blueprints/3DCraneDDeliverInterface.DeliverData` (`self.FakeData2`) _x _x 0.0 _a _a))
    (:`Finished`
      (`self.SendMore`))))

(event `SendMore`
  ;[1 1 1] Probably made for some kind of test
  (`/Engine/EditorBlueprintResources/StandardMacros.FlipFlop`
    (:`A`
      (goto _label :!via `Reverse`))
    (:`B`
      (goto _label :!via `PlayFromStart`))))

(fn `UserConstructionScript`)