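; MLS UDP receiver actor that relays height, lateral movement and external SP values to an MLS implementation through DeliverDataMessage.
; Tick forwards new socket data when the receive socket is ready, but the localhost socket startup is disconnected and never runs.
; BeginPlay instead starts the FakeData timeline, which sends simulated height and X values to two targets and ping-pongs endlessly via a FlipFlop on finish.
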(event `self.ReceiveTick`
  (params (DeltaSeconds :type "Float (single-precision)"))
  (if (`self.RcvSocketReady`)
    (bind _returnvalue (`self.IsNewDataReady`))
    (if _returnvalue
      (bind _returnvalue_2 (`self.GetData`))
      (bind (_float1 _float2 _float3 _float4) (break `UDPData` _returnvalue_2))
      (message `/Game/Blueprints/MLSDDeliverInterface.DeliverData` (`self.MLSImplRef`) _float1 _float2 _float3 _float4))))

(event `SendMore`
  (`/Engine/EditorBlueprintResources/StandardMacros.FlipFlop`
    (:`A`
      (bind (_direction _hight _x) (`Timeline|FakeData` :!via `Reverse` :!label _label)
        (:`Update`
          (message `/Game/Blueprints/MLSDDeliverInterface.DeliverData` (`self.SendFakeData`) _hight _x 0.0 0.0)
          (message `/Game/Blueprints/MLSDDeliverInterface.DeliverData` (`self.SendFakeData2`) _hight _x 0.0 0.0))
        (:`Finished`
          (`self.SendMore`))))
    (:`B`
      (goto _label :!via `PlayFromStart`))))

(event `self.ReceiveBeginPlay`
  (goto _label))

(fn `UserConstructionScript`)