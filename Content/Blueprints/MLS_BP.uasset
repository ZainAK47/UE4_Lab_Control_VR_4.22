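; VR front end for an MLS magnetic levitation rig, exchanging data over UDP and moving the ball from delivered height and lateral values.
; Trigger-held laser traces against a reference cube map through a spline to a height setpoint and crosshair.
; Controller touches turn hand motion into timed lateral impulses with haptics.
; Tick sends setpoint, selected mode and disturbances; a looping timer feeds actual and desired heights to graph widgets.
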(event `PlayAnimation`
  (params (`Fwd/Back` :type Boolean))
  (bind _crosshair (`self.Crosshair`))
  ;[1 1 1] Timeline Animation
  (if `Fwd/Back`
    (bind (_direction _alpha) (`Timeline|Timeline_0` :!via `PlayFromStart` :!label _label)
      (:`Update`
        (`SceneComponent.SetRelativeScale3D` _crosshair (`KismetMathLibrary.VLerp` (0.1 0.1 0.1) (0.03 0.03 0.03) _alpha))
        (`MeshComponent.SetScalarParameterValueOnMaterials` _crosshair "TheOpacity" (`KismetMathLibrary.Lerp` 0.0 0.9 _alpha))))
    (else
      (goto _label :!via `Reverse`))))

(event `self.mls-ball-only_optimized.OnComponentBeginOverlap`
  (params (OverlappedComponent :type "PrimitiveComponent Object Reference") (OtherActor :type "Actor Object Reference") (OtherComp :type "PrimitiveComponent Object Reference") (OtherBodyIndex :type Integer) (bFromSweep :type Boolean) (SweepResult :type "HitResult Structure (by ref)"))
  (`self.BallBeginOverlappingWith` OtherActor))

(event `self.mls-ball-only_optimized.OnComponentEndOverlap`
  (params (OverlappedComponent :type "PrimitiveComponent Object Reference") (OtherActor :type "Actor Object Reference") (OtherComp :type "PrimitiveComponent Object Reference") (OtherBodyIndex :type Integer))
  (`self.BallEndOverlappingWith` OtherActor))

(event `self.ReceiveBeginPlay`
  (bind _mls_cuberef (`self.MLS_cubeRef`))
  (bind _motioncontrolledpawn (`self.MotionControlledPawn`))
  (bind _outactors (`GameplayStatics.GetAllActorsOfClass` "/Game/VirtualRealityBP/Blueprints/MotionControllerPawn.MotionControllerPawn_C"))
  (bind _output (`|GetArrayItem` _outactors))
  (`/Engine/EditorBlueprintResources/StandardMacros.IsValid` _output
    (:`Is Valid`
      (set `self.MotionControlledPawn` _output)
      (bind _outactors_2 (`GameplayStatics.GetAllActorsOfClass` "/Game/Blueprints/FreeCamera.FreeCamera_C"))
      (bind _output_2 (`|GetArrayItem` _outactors_2))
      (`/Engine/EditorBlueprintResources/StandardMacros.IsValid` _output_2
        (:`Is Valid`
          (set `self.FreeCamRef` _output_2)
          (bind _outactors_3 (`GameplayStatics.GetAllActorsOfClass` "/Game/Blueprints/MLSUDPReceiver.MLSUDPReceiver_C"))
          (bind _output_3 (`|GetArrayItem` _outactors_3))
          (`/Engine/EditorBlueprintResources/StandardMacros.IsValid` _output_3
            (:`Is Valid`
              (set `self.UDP_Receiver` _output_3)
              (bind _outactors_4 (`GameplayStatics.GetAllActorsOfClass` "/Game/Blueprints/MLSUDPSender.MLSUDPSender_C"))
              (bind _output_4 (`|GetArrayItem` _outactors_4))
              (`/Engine/EditorBlueprintResources/StandardMacros.IsValid` _output_4
                (:`Is Valid`
                  (set `self.MLSUDPSender` _output_4)
                  (bind _outactors_5 (`GameplayStatics.GetAllActorsOfClass` "/Game/Blueprints/MLS_Ref_Cube.MLS_Ref_Cube_C"))
                  (bind _output_5 (`|GetArrayItem` _outactors_5))
                  (`/Engine/EditorBlueprintResources/StandardMacros.IsValid` _output_5
                    (:`Is Valid`
                      (set `self.MLS_cubeRef` _output_5)
                      (set `self.RefCube` (`|GetArrayItem` (`self.GetComponentsByTag` _mls_cuberef "/Script/Engine.StaticMeshComponent" "MLSCube")))
                      (set `self.Crosshair` (`|GetArrayItem` (`self.GetComponentsByTag` _mls_cuberef "/Script/Engine.StaticMeshComponent" "Crosshair")))
                      (set `self.SplineRef` (`|GetArrayItem` (`self.GetComponentsByTag` _mls_cuberef "/Script/Engine.SplineComponent" "spline"))))
                    (:`Is Not Valid`
                      (bind _outactors_6 (`GameplayStatics.GetAllActorsWithTag` "Crosshair"))
                      (bind _output_6 (`|GetArrayItem` _outactors_6))
                      (`/Engine/EditorBlueprintResources/StandardMacros.IsValid` _output_6
                        (:`Is Valid`
                          (set `self.CrosshairRef` _output_6))
                        (:`Is Not Valid`
                          _))
                      (bind _outactors_7 (`GameplayStatics.GetAllActorsWithTag` "MLSCube"))
                      (bind _output_7 (`|GetArrayItem` _outactors_7))
                      (`/Engine/EditorBlueprintResources/StandardMacros.IsValid` _output_7
                        (:`Is Valid`
                          (set `self.MLSCubeRef` _output_7))
                        (:`Is Not Valid`
                          _))))
                  ;[1 1 1] macros
                  (`self.InitializeSetPointLocation`)
                  (`self.InitializeUDPComms`)
                  (bind _outactors_8 (`GameplayStatics.GetAllActorsOfClass` "/Game/Blueprints/Widget_BP/MovableWidget_BP.MovableWidget_BP_C"))
                  (for _array_element _outactors_8
                    (bind _asmovable_widget_bp (cast `/Game/Blueprints/Widget_BP/MovableWidget_BP` _array_element))
                    (bind _returnvalue (`WidgetComponent.GetUserWidgetObject` (`/Game/Blueprints/Widget_BP/MovableWidget_BP.Widget` _asmovable_widget_bp)))
                    (if (== (`GameplayStatics.GetObjectClass` _returnvalue) "/Game/Blueprints/Widget_BP/RealGraph_Widget.RealGraph_Widget_C")
                      (bind _asreal_graph_widget (cast `/Game/Blueprints/Widget_BP/RealGraph_Widget` _returnvalue))
                      (`KismetArrayLibrary.Array_Add` (`self.GraphWidgets`) _asreal_graph_widget)))
                  (`|ExecutionSequence`
                    (:`then_0`
                      (add `/Game/VirtualRealityBP/Blueprints/MotionControllerPawn.RightTriggerPress` _motioncontrolledpawn (delegate `RTP`))
                      (add `/Game/VirtualRealityBP/Blueprints/MotionControllerPawn.RightTriggerRelease` _motioncontrolledpawn (delegate `RTRlease`))
                      (`KismetSystemLibrary.K2_SetTimerDelegate` (delegate `AddData`) 0.01 true))))))))))))

(event `AddData`
  (for _array_element (`self.GraphWidgets`)
    (`/Game/Blueprints/Widget_BP/RealGraph_Widget.AddActualHeight` _array_element (`self.TheHeight`))
    (`/Game/Blueprints/Widget_BP/RealGraph_Widget.AddDesiredHeight` _array_element (`self.TheExternalSP`))))

(event `RTP`
  (`self.RT_Press`))

(event `RTRlease`
  (`self.RT_Release`))

(event `BallBeginOverlappingWith`
  (params (OtherActor :type "Actor Object Reference"))
  (bind (_x _y) (`self.DisturbanceTouchLogic` OtherActor (stale `BallEndOverlappingWith` OtherActor) :!label _label)
    (:`BeginOverlap`
      (bind (_direction _impulse) (`Timeline|GenerateImpulse` :!label _label_2)
        (:`Update`
          (set `self.LateralDistX` (* _impulse _x))
          (set `self.LateralDistY` (* _impulse _y)))))
    (:`EndOverlap`
      (`|ExecutionSequence`
        (:`then_0`
          (goto _label_2 :!via `Stop`))
        (:`then_1`
          (goto _label_2 :!via `SetNewTime`))))))

(event `BallEndOverlappingWith`
  (params (OtherActor :type "Actor Object Reference"))
  (goto _label :!via `EndControllerOverlapEvent`))

(event `Key|Ctrl+NumPadOne` :consume false
  (params (Key :type "Key Structure"))
  (bind _returnvalue (`GameplayStatics.GetGameInstance`))
  (bind (_text_mlsmode0 _text_mlsmode1) (break `/Game/Blueprints/UserMsgs` (`self.ModeStruct`)))
  ;[1 1 1] Vive and Freecamera mode switching
  (:`Pressed`
    (`/Engine/EditorBlueprintResources/StandardMacros.FlipFlop` :!label _label
      (:`A`
        (bind _output_get (set `self.OperationMode` 1))
        (bind _asglobal_variables (cast `/Game/ControllersWithGuides/GlobalVariables` _returnvalue)) ; For Text indication
        (set `/Game/ControllersWithGuides/GlobalVariables.CurrentMode` _output_get _asglobal_variables)
        (bind (_direction _opacitytrack) (`Timeline|TimelineDisplayText` :!label _label_2) ; Does this even work anymore?
          (:`Update`
            (`self.UpdateMessageWidgetRight` (select `byte` (`self.OperationMode`) :`0` _text_mlsmode0 :`1` _text_mlsmode1) _opacitytrack :!label _label_3))
          (:`Finished`
            (goto _label_3 :!via `DisableText`))))
      (:`B`
        (bind _output_get_2 (set `self.OperationMode` 0))
        (bind _asglobal_variables_2 (cast `/Game/ControllersWithGuides/GlobalVariables` _returnvalue))
        (set `/Game/ControllersWithGuides/GlobalVariables.CurrentMode` _output_get_2 _asglobal_variables_2)
        (goto _label_2)))))

(event `InputAction|ModeSwitch` :consume false
  (params (Key :type "Key Structure"))
  ;[1 1 1] Vive and Freecamera mode switching
  (:`Pressed`
    (goto _label)))

(event `Key|MotionController_Right_FaceButton2` :consume false :overrideparent false
  (params (Key :type "Key Structure"))
  ;[1 1 1] Oculus controllers custom selection
  (:`Pressed`
    (bind _output_get (set `self.OperationMode` 0))
    (bind _asglobal_variables (cast `/Game/ControllersWithGuides/GlobalVariables` (`GameplayStatics.GetGameInstance`))) ; For text indication (not done on oculus yet)
    (set `/Game/ControllersWithGuides/GlobalVariables.CurrentMode` _output_get _asglobal_variables)
    (goto _label_2)))

(event `Key|MotionController_Right_FaceButton1` :consume false :overrideparent false
  (params (Key :type "Key Structure"))
  ;[1 1 1] Oculus controllers custom selection
  (:`Pressed`
    (bind _output_get (set `self.OperationMode` 1))
    (bind _asglobal_variables (cast `/Game/ControllersWithGuides/GlobalVariables` (`GameplayStatics.GetGameInstance`)))
    (set `/Game/ControllersWithGuides/GlobalVariables.CurrentMode` _output_get _asglobal_variables)
    (goto _label_2)))

(event `RT_Press`
  (`|ExecutionSequence` :!label _label
    (:`then_0`
      (set `self.IsTrackingEnabled` true))
    (:`then_1`
      (`SceneComponent.SetVisibility` (`/Game/VirtualRealityBP/Blueprints/BP_MotionController.GreenLaserBeam` (`/Game/VirtualRealityBP/Blueprints/MotionControllerPawn.RightController` (`self.MotionControlledPawn`))) true false)
      (`self.PlayAnimation` true))))

(event `Key|LeftMouseButton` :consume false
  (params (Key :type "Key Structure"))
  (:`Pressed`
    (goto _label))
  (:`Released`
    (set `self.IsTrackingEnabled` false :!label _label_2)
    (`SceneComponent.SetVisibility` (`/Game/VirtualRealityBP/Blueprints/BP_MotionController.GreenLaserBeam` (`/Game/VirtualRealityBP/Blueprints/MotionControllerPawn.RightController` (`self.MotionControlledPawn`))) false false)
    (`self.PlayAnimation` false)))

(event `RT_Release`
  (goto _label_2))

(event `self.ReceiveTick`
  (params (DeltaSeconds :type "Float (single-precision)"))
  (bind _arcdirection (`/Game/VirtualRealityBP/Blueprints/BP_MotionController.ArcDirection` (`/Game/VirtualRealityBP/Blueprints/MotionControllerPawn.RightController` (`self.MotionControlledPawn`))))
  (bind _greenlaserbeam (`/Game/VirtualRealityBP/Blueprints/BP_MotionController.GreenLaserBeam` (`/Game/VirtualRealityBP/Blueprints/MotionControllerPawn.RightController` (`self.MotionControlledPawn`))))
  (bind _returnvalue (`SceneComponent.K2_GetComponentLocation` _arcdirection))
  (bind _returnvalue_2 (* (`SceneComponent.GetForwardVector` _arcdirection) 1500000.0))
  (`|ExecutionSequence`
    (:`then_0`
      (if (`self.IsTrackingEnabled`)
        (bind _location (`self.TestReferenceCubeHit` _returnvalue _returnvalue_2)
          (:`true`
            (`self.SetSPAndDrawCrosshair` _location)))))
    (:`then_1`
      (message `/Game/Blueprints/MLSDSendInterface.SendData` (`self.MLSUDPSender`) (`self.SPHeight`) (`self.OperationMode`) (`self.LateralDistX`) (`self.LateralDistY`)))
    (:`then_2`
      (`ParticleSystemComponent.SetBeamSourcePoint` _greenlaserbeam 0 _returnvalue 0)
      (`ParticleSystemComponent.SetBeamTargetPoint` _greenlaserbeam 0 _returnvalue_2 0)
      (`SceneComponent.K2_AddLocalRotation` (`self.Crosshair`) (struct :`Roll` 1.0) false false))
    (:`then_3`
      (`self.GetControllerDynamics`))))

(event `/Game/Blueprints/MLSDDeliverInterface.DeliverData`
  (params (CurrentHeight :type "Float (single-precision)") (LateralMovementX :type "Float (single-precision)") (LateralMovementY :type "Float (single-precision)") (ExternalSP :type "Float (single-precision)"))
  (`SceneComponent.K2_SetRelativeLocation` (`self.mls-ball-only_optimized`) (`KismetMathLibrary.MakeVector` (* LateralMovementX 2.5) (* LateralMovementY 2.5) (- 2.0 (* 2.0 (/ CurrentHeight (`self.MaxDistFromMagnet`))))) false false)
  (set `self.TheHeight` CurrentHeight)
  (set `self.TheExternalSP` ExternalSP))

(fn `UserConstructionScript`)