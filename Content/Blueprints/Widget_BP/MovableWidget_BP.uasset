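; VR actor wrapping a Graph_Widget panel that motion controllers can grab, move, resize and throw.
; The first hand attaches the actor; while a second hand also overlaps the widget, Tick scales Y and Z from changes in hand distance, within limits.
; Dropping outside the Widget_Socket_BP compares position with the last tick's to detect a throw.
; Thrown widgets simulate physics temporarily, then reattach to their root and return to the socket's display.
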(event `self.ReceiveBeginPlay`
  ;[1 1 1] Begin play
  (bind _outactors (`GameplayStatics.GetAllActorsOfClass` "/Game/VirtualRealityBP/Blueprints/MotionControllerPawn.MotionControllerPawn_C"))
  (set `self.MotionControllerPawn_Ref` (`|GetArrayItem` _outactors))
  (bind _outactors_2 (`GameplayStatics.GetAllActorsOfClass` "/Game/Blueprints/Widget_BP/Widget_Socket_BP.Widget_Socket_BP_C"))
  (set `self.Widget_Socket_Ref` (`|GetArrayItem` _outactors_2))
  (bind _asgraph_widget (cast `/Game/Blueprints/Widget_BP/Graph_Widget` (`WidgetComponent.GetUserWidgetObject` (`self.Widget`))))
  (set `/Game/Blueprints/Widget_BP/Graph_Widget.Docked` false _asgraph_widget))

(event `/Game/VirtualRealityBP/Blueprints/PickupActorInterface.Pickup`
  (params (AttachTo :type "SceneComponent Object Reference"))
  ;[1 1 1] Pickup
  (if (`self.WasThrowed`)
    _
    (elif (`self.InUse`)
      (set `self.SecondHand` AttachTo)
      (`self.SetActorTickEnabled` true)
      (else
        (set `self.InUse` true)
        (if (`KismetSystemLibrary.IsValid` AttachTo)
          (bind _output_get (set `self.FirstHand` AttachTo))
          (set `self.SecondHand` null)
          (`self.SetActorTickEnabled` true)
          (`self.K2_AttachToComponent` _output_get "None" "KeepWorld" "KeepWorld" "KeepWorld"))))))

(event `/Game/VirtualRealityBP/Blueprints/PickupActorInterface.Drop`
  (params (DeatacthFrom :type "SceneComponent Object Reference"))
  (bind _returnvalue (`self.K2_GetActorLocation`))
  (bind _oldframepos (`self.OldFramePos`))
  (bind _widget (`self.Widget`))
  ;[1 1 1] Drop
  (if (== DeatacthFrom (`self.FirstHand`))
    (set `self.InUse` false)
    (if (`KismetArrayLibrary.Array_Contains` (`self.GetOverlappingActors` (`self.Widget_Socket_Ref`) "MovableWidget_BP_C") self)
      (`|ExecutionSequence`
        (:`then_0`
          (`self.SetActorTickEnabled` false :!label _label)
          (set `self.SecondHand` null :!label _label_2))
        (:`then_1`
          (set `self.FirstHand` null :!label _label_3)
          (`self.K2_DetachFromActor` "KeepWorld" "KeepWorld" "KeepWorld")))
      (else
        (`|ExecutionSequence`
          (:`then_0`
            (goto _label))
          (:`then_1`
            (if (and (!= _oldframepos (0.0 0.0 0.0) :`ErrorTolerance` 0.0) (!= _returnvalue (0.0 0.0 0.0) :`ErrorTolerance` 0.0))
              (if (> (/ (`KismetMathLibrary.Vector_Distance` _returnvalue _oldframepos) (`self.TickDeltaSeconds`)) 150.0)
                (set `self.WasThrowed` true)
                (`PrimitiveComponent.SetSimulatePhysics` (`self.Widget`) true)
                ;[1 1 1] Widget throwing
                (`|ExecutionSequence`
                  (:`then_0`
                    (goto _label_3))
                  (:`then_1`
                    (`KismetSystemLibrary.Delay` (`self.DurationOfPhysicForm`))
                    (`PrimitiveComponent.SetSimulatePhysics` (`self.Widget`) false)
                    (set `self.WasThrowed` false)
                    (set `self.TickDeltaSeconds` 0.0)
                    (`self.SetActorTickEnabled` false)
                    (`SceneComponent.K2_AttachToComponent` _widget (`self.Scene`) "None" "KeepRelative" "KeepRelative" "KeepRelative" true)
                    (`SceneComponent.K2_SetRelativeLocationAndRotation` :`self` _widget :`NewLocation` (2.599986 -0.542494 21.787319))
                    (`SceneComponent.SetRelativeScale3D` _widget (0.2 0.035 0.04375))
                    (set `self.OldFramePos` (`self.K2_GetActorLocation`))
                    (`self.AddToDisplayManualy` (`self.Widget_Socket_Ref`) self)))
                (else
                  (goto _label_3))))))))
    (else
      (goto _label_2))))

(event `self.ReceiveTick`
  (params (DeltaSeconds :type "Float (single-precision)"))
  (bind _widgetminscale (`self.WidgetMinScale`))
  (bind _widgetmaxscale (`self.WidgetMaxScale`))
  (bind _widgetscalingspeed (`self.WidgetScalingSpeed`))
  (bind _secondhand (`self.SecondHand`))
  (bind _firsthand (`self.FirstHand`))
  (bind _secondhand_2 (`self.SecondHand`))
  (bind _widget (`self.Widget`))
  (bind _returnvalue (`KismetMathLibrary.Vector_Distance` (`SceneComponent.K2_GetComponentLocation` _secondhand) (`SceneComponent.K2_GetComponentLocation` (`self.FirstHand`))))
  ;[1 1 1] Widget scaling
  (if (`KismetSystemLibrary.IsValid` (`self.SecondHand`))
    (if (and (`KismetSystemLibrary.IsValid` _firsthand) (`KismetSystemLibrary.IsValid` _secondhand_2))
      (if (and (`PrimitiveComponent.IsOverlappingActor` _widget (`ActorComponent.GetOwner` _firsthand)) (`PrimitiveComponent.IsOverlappingActor` _widget (`ActorComponent.GetOwner` _secondhand_2)))
        (if (`KismetSystemLibrary.IsValid` _secondhand)
          (if (!= (`self.Distance`) 0.0)
            (if (not (`KismetMathLibrary.NearlyEqual_FloatFloat` (stale _output_get) _returnvalue 1.0))
              (bind _returnvalue_2 (select `bool` (> _returnvalue (stale _output_get)) :`false` (* (/ _returnvalue _widgetscalingspeed) -1.0) :`true` (/ _returnvalue _widgetscalingspeed)))
              (`self.SetActorScale3D` (`KismetMathLibrary.MakeVector` (.x (`self.GetActorScale3D`)) (`KismetMathLibrary.FClamp` (+ (.y (`self.GetActorScale3D`)) _returnvalue_2) _widgetminscale _widgetmaxscale) (`KismetMathLibrary.FClamp` (+ (.z (`self.GetActorScale3D`)) _returnvalue_2) _widgetminscale _widgetmaxscale)))
              (set `self.Distance` _returnvalue))
            (else
              (bind _output_get (set `self.Distance` _returnvalue)))))))
    (else
      (set `self.TickDeltaSeconds` DeltaSeconds)
      (set `self.OldFramePos` (`self.K2_GetActorLocation`)))))

(fn `UserConstructionScript`)