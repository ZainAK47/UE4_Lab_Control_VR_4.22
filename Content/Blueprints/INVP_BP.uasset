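; VR inverted pendulum on a cart, driven by data exchanged over local UDP.
; Holding right grab aims a laser trace that snaps a marker along the track and sets the cart setpoint.
; Right-controller contact yields a disturbance from hand movement, signed by spline side, with haptic clicks.
; Tick sends setpoint, disturbance and toggleable control mode through the sender; DeliverData applies cart position and pendulum angle to the meshes.
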(event `PlayAnimation`
  (params (`Fwd/Back` :type Boolean))
  (bind _thesp (`self.TheSP`))
  ;[1 1 1] TimelineAnimation
  (if `Fwd/Back`
    (bind (_direction _alpha) (`Timeline|CylAnimation` :!via `PlayFromStart` :!label _label)
      (:`Update`
        (`SceneComponent.SetRelativeScale3D` _thesp (`KismetMathLibrary.VLerp` (0.4 0.4 0.02) (0.25 0.25 0.02) _alpha))
        (`MeshComponent.SetScalarParameterValueOnMaterials` _thesp "TheOpacity" (`KismetMathLibrary.Lerp` _alpha 0.0 0.7))))
    (else
      (goto _label :!via `Reverse`))))

(event `self.ReceiveBeginPlay`
  (bind _outactors (`GameplayStatics.GetAllActorsOfClass` "/Game/VirtualRealityBP/Blueprints/MotionControllerPawn.MotionControllerPawn_C"))
  (bind _output (`|GetArrayItem` _outactors))
  (`/Engine/EditorBlueprintResources/StandardMacros.IsValid` _output
    (:`Is Valid`
      (set `self.MotionControlledPawn` _output)
      (bind _outactors_2 (`GameplayStatics.GetAllActorsOfClass` "/Game/Blueprints/FreeCamera.FreeCamera_C"))
      (bind _output_2 (`|GetArrayItem` _outactors_2))
      (`/Engine/EditorBlueprintResources/StandardMacros.IsValid` _output_2
        (:`Is Valid`
          (set `self.FreeCamRef` _output_2)
          (bind _outactors_3 (`GameplayStatics.GetAllActorsOfClass` "/Game/Blueprints/InvpCommandSenderUDP.InvpCommandSenderUDP_C"))
          (bind _output_3 (`|GetArrayItem` _outactors_3))
          (`/Engine/EditorBlueprintResources/StandardMacros.IsValid` _output_3
            (:`Is Valid`
              (set `self.InvpCommandSenderUDP` _output_3)
              (bind _outactors_4 (`GameplayStatics.GetAllActorsOfClass` "/Game/Blueprints/InvpCommandReceiverUDP.InvpCommandReceiverUDP_C"))
              (bind _output_4 (`|GetArrayItem` _outactors_4))
              (`/Engine/EditorBlueprintResources/StandardMacros.IsValid` _output_4
                (:`Is Valid`
                  (set `self.InvpCommandReceiverUDP` _output_4)
                  (`self.InitializeUDPComms`)
                  (set `self.OriginalCaretLocation` (`SceneComponent.RelativeLocation` (`self.Kareta`)))
                  (set `self.OriginalPendulumRotation` (`SceneComponent.RelativeRotation` (`self.Pendulum`))))))))))))

(event `Key|Ctrl+NumPadOne` :consume false
  (params (Key :type "Key Structure"))
  ;[1 1 1] ModeSwitcher
  (:`Pressed`
    (`/Engine/EditorBlueprintResources/StandardMacros.FlipFlop` :!label _label
      (:`A`
        (set `self.PendulumControlMode` 0))
      (:`B`
        (set `self.PendulumControlMode` 1)))))

(event `InputAction|ModeSwitch` :consume false
  (params (Key :type "Key Structure"))
  ;[1 1 1] ModeSwitcher
  (:`Pressed`
    (goto _label)))

(event `self.staticm.OnComponentBeginOverlap`
  (params (OverlappedComponent :type "PrimitiveComponent Object Reference") (OtherActor :type "Actor Object Reference") (OtherComp :type "PrimitiveComponent Object Reference") (OtherBodyIndex :type Integer) (bFromSweep :type Boolean) (SweepResult :type "HitResult Structure (by ref)"))
  (bind _rightcontroller (`/Game/VirtualRealityBP/Blueprints/MotionControllerPawn.RightController` (`self.MotionControlledPawn`)))
  ;[1 1 1] Disturbance Overlap
  (if (== OtherComp (`/Game/VirtualRealityBP/Blueprints/BP_MotionController.INVPCol` _rightcontroller))
    (set `self.Overlaping` true)
    (`PlayerController.PlayHapticEffect` (`GameplayStatics.GetPlayerController` 0) "/Game/VirtualRealityBP/Blueprints/TouchClick.TouchClick" (`/Game/VirtualRealityBP/Blueprints/BP_MotionController.Hand` _rightcontroller) 1.0 false :!label _label_2)))

(event `self.staticm.OnComponentEndOverlap`
  (params (OverlappedComponent :type "PrimitiveComponent Object Reference") (OtherActor :type "Actor Object Reference") (OtherComp :type "PrimitiveComponent Object Reference") (OtherBodyIndex :type Integer))
  ;[1 1 1] Disturbance Overlap
  (if (== OtherComp (`/Game/VirtualRealityBP/Blueprints/BP_MotionController.INVPCol` (`/Game/VirtualRealityBP/Blueprints/MotionControllerPawn.RightController` (`self.MotionControlledPawn`))))
    (set `self.PendulumDisturbance` 0.0)
    (set `self.Overlaping` false)
    (goto _label_2)))

(event `self.ReceiveTick`
  (params (DeltaSeconds :type "Float (single-precision)"))
  (bind _track (`self.Track`))
  (bind (_drightcontrollerlocation_x _drightcontrollerlocation_y _drightcontrollerlocation_z) (`KismetMathLibrary.BreakVector` (`self.dRightControllerLocation`)))
  (bind _arcdirection (`/Game/VirtualRealityBP/Blueprints/BP_MotionController.ArcDirection` (`/Game/VirtualRealityBP/Blueprints/MotionControllerPawn.RightController` (`self.MotionControlledPawn`))))
  (bind _greenlaserbeam (`/Game/VirtualRealityBP/Blueprints/BP_MotionController.GreenLaserBeam` (`/Game/VirtualRealityBP/Blueprints/MotionControllerPawn.RightController` (`self.MotionControlledPawn`))))
  (bind _returnvalue (`SceneComponent.K2_GetComponentLocation` (`/Game/VirtualRealityBP/Blueprints/BP_MotionController.ArcDirection` (`/Game/VirtualRealityBP/Blueprints/MotionControllerPawn.RightController` (`self.MotionControlledPawn`)))))
  (bind _returnvalue_2 (`SceneComponent.K2_GetComponentLocation` _arcdirection))
  (bind _returnvalue_3 (* (`SceneComponent.GetForwardVector` _arcdirection) 1500000.0))
  (`|ExecutionSequence`
    (:`then_0`
      (if (`self.IsTrackingEnabled`)
        (bind _outhit (`KismetSystemLibrary.LineTraceSingle` _returnvalue_2 _returnvalue_3 "TraceTypeQuery1" false (`|MakeArray` (`ChildActorComponent.ChildActor` (`/Game/VirtualRealityBP/Blueprints/BP_MotionController.MyUserMessage` (`/Game/VirtualRealityBP/Blueprints/MotionControllerPawn.RightController` (`self.MotionControlledPawn`))))) "ForOneFrame" false))
        (bind (_bblockinghit _binitialoverlap _time _distance _location _impactpoint _normal _impactnormal _physmat _hitactor _hitcomponent) (`GameplayStatics.BreakHitResult` _outhit))
        (if (== _hitcomponent (`self.BoxCol`))
          (set `self.CaretSetPoint` (`KismetMathLibrary.Lerp` 1.89 0.0 (`SplineComponent.FindInputKeyClosestToWorldLocation` _track _location)))
          (`SceneComponent.K2_SetWorldLocation` (`self.TheSP`) (`SplineComponent.FindLocationClosestToWorldLocation` _track _location "World") false false))))
    (:`then_1`
      (message `/Game/Blueprints/InvpDSendInterface.InvpDeliverSendData` (`self.InvpCommandSenderUDP`) (`self.CaretSetPoint`) (`self.PendulumDisturbance`) (`self.PendulumControlMode`)))
    (:`then_2`
      (`ParticleSystemComponent.SetBeamSourcePoint` _greenlaserbeam 0 _returnvalue_2 0)
      (`ParticleSystemComponent.SetBeamTargetPoint` _greenlaserbeam 0 _returnvalue_3 0))
    (:`then_3`
      ;[1 1 1] Controller speed
      (set `self.dRightControllerLocation` (- _returnvalue (`self.RightControllerLocation`)))
      (set `self.RightControllerLocation` _returnvalue)
      ;[1 1 1] DIsturbance force
      (if (> (`SplineComponent.FindInputKeyClosestToWorldLocation` (`self.Spline`) (`SceneComponent.K2_GetComponentLocation` (`/Game/VirtualRealityBP/Blueprints/BP_MotionController.INVPCol` (`/Game/VirtualRealityBP/Blueprints/MotionControllerPawn.RightController` (`self.MotionControlledPawn`))))) 0.5)
        (set `self.DistMultiplier` 3.0)
        (else
          (set `self.DistMultiplier` -3.0)))
      (if (`self.Overlaping`)
        (bind _output_get (set `self.PendulumDisturbance` (* (+ (`KismetMathLibrary.Abs` _drightcontrollerlocation_x) (`KismetMathLibrary.Abs` _drightcontrollerlocation_y) (`KismetMathLibrary.Abs` _drightcontrollerlocation_z)) (`self.DistMultiplier`))))
        (if (> (`KismetMathLibrary.Abs` _output_get) 5.0)
          (`KismetSystemLibrary.PrintString` (`KismetStringLibrary.Conv_DoubleToString` _output_get)))
        (else
          (set `self.PendulumDisturbance` 0.0))))))

(event `InputAction|GrabRight` :consume false
  (params (Key :type "Key Structure"))
  (bind _greenlaserbeam (`/Game/VirtualRealityBP/Blueprints/BP_MotionController.GreenLaserBeam` (`/Game/VirtualRealityBP/Blueprints/MotionControllerPawn.RightController` (`self.MotionControlledPawn`))))
  (:`Pressed`
    (`|ExecutionSequence`
      (:`then_0`
        (set `self.IsTrackingEnabled` true))
      (:`then_1`
        (`SceneComponent.SetVisibility` _greenlaserbeam true false))
      (:`then_2`
        (`self.PlayAnimation` true))))
  (:`Released`
    (`|ExecutionSequence`
      (:`then_0`
        (set `self.IsTrackingEnabled` false)
        (`SceneComponent.SetVisibility` _greenlaserbeam false false))
      (:`then_1`
        (`self.PlayAnimation` false)))))

(event `/Game/Blueprints/InvpDDeliverInterface.DeliverData`
  (params (CaretPosition :type "Float (single-precision)") (PendulumAngle :type "Float (single-precision)"))
  (`SceneComponent.K2_SetRelativeLocation` (`self.Kareta`) (`KismetMathLibrary.MakeVector` (+ (.x (`self.OriginalCaretLocation`)) (* CaretPosition -1.0)) (.y (`self.OriginalCaretLocation`)) (.z (`self.OriginalCaretLocation`))) false false)
  (`SceneComponent.K2_SetRelativeRotation` (`self.Pendulum`) (`KismetMathLibrary.MakeRotator` (.roll (`self.OriginalPendulumRotation`)) (+ (.pitch (`self.OriginalPendulumRotation`)) (`KismetMathLibrary.RadiansToDegrees` PendulumAngle)) (.yaw (`self.OriginalPendulumRotation`))) false false))

(fn `UserConstructionScript`)