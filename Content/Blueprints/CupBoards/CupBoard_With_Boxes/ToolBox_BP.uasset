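; Toolbox actor with a sliding shelf that is grabbed by a controller component and moved along a single axis.
; While held, Tick projects the controller's position onto the X-axis line and clamps the shelf between its travel limits.
; Drop estimates release speed from the last frame's movement, and fast releases glide on with per-frame decay that is not scaled by delta time.
; Tick is enabled on pickup and disabled once the shelf settles.
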(event `/Game/VirtualRealityBP/Blueprints/PickupActorInterface.Pickup`
  (params (AttachTo :type "SceneComponent Object Reference"))
  ;[1 1 1] Pickup event
  (if (`KismetSystemLibrary.IsValid` AttachTo)
    (if (`self.autoMovement`)
      (set `self.autoMovement` false)
      (set `self.TickDeltaSeconds` 0.0)
      (set `self.MovementSpeedToMaxPos` 0.0)
      (set `self.OldBoxPosition` 0.0)
      (set `self.ChangeValueMov` 0.0))
    (set `self.ControllerToAttach` AttachTo)
    (`self.SetActorTickEnabled` true)))

(event `/Game/VirtualRealityBP/Blueprints/PickupActorInterface.Drop`
  (params (DeatacthFrom :type "SceneComponent Object Reference"))
  (bind _controllertoattach (`self.ControllerToAttach`))
  (bind _relativelocation (`SceneComponent.RelativeLocation` (`self.Scene`)))
  (bind _returnvalue (/ (- (`self.OldBoxPosition`) (.x (- (`KismetMathLibrary.FindClosestPointOnLine` (`SceneComponent.RelativeLocation` (`self.ControllerScene`)) _relativelocation (-1.0 0.0 0.0)) _relativelocation))) (`self.TickDeltaSeconds`)))
  ;[1 1 1] Drop event
  (if (`KismetSystemLibrary.IsValid` _controllertoattach)
    (if (== _controllertoattach DeatacthFrom)
      (if (or (> _returnvalue 25.0) (< _returnvalue -25.0))
        (set `self.MovementSpeedToMaxPos` (* _returnvalue -1.0))
        (set `self.ControllerToAttach` null)
        (set `self.autoMovement` true)
        (else
          (set `self.ControllerToAttach` null)
          (`self.SetActorTickEnabled` false))))))

(event `self.ReceiveTick`
  (params (DeltaSeconds :type "Float (single-precision)"))
  (bind _movementspeedtomaxpos (`self.MovementSpeedToMaxPos`))
  (bind _sm_toolbox_shelf (`self.SM_Toolbox_Shelf`))
  (bind _sm_toolbox_shelf_2 (`self.SM_Toolbox_Shelf`))
  (bind _relativelocation (`SceneComponent.RelativeLocation` (`self.Scene`)))
  (bind _x (.x (- (`KismetMathLibrary.FindClosestPointOnLine` (`SceneComponent.RelativeLocation` (`self.ControllerScene`)) _relativelocation (-1.0 0.0 0.0)) _relativelocation)))
  (if (`self.autoMovement`)
    ;[1 1 1] Toolbox physics
    (bind _output_get (set `self.ChangeValueMov` (+ (/ _movementspeedtomaxpos 50.0) (`self.ChangeValueMov`))))
    (`SceneComponent.K2_SetRelativeLocation` _sm_toolbox_shelf_2 (`KismetMathLibrary.MakeVector` (`KismetMathLibrary.FClamp` (+ _x _output_get) (`self.MaxPosition`) (`self.MinPosition`)) (.y (`SceneComponent.RelativeLocation` _sm_toolbox_shelf_2)) (.z (`SceneComponent.RelativeLocation` _sm_toolbox_shelf_2))) false false)
    (bind _output_get_2 (set `self.MovementSpeedToMaxPos` (/ _movementspeedtomaxpos 1.1)))
    (if (`KismetMathLibrary.NearlyEqual_FloatFloat` _output_get_2 0.0 1.0)
      (set `self.ControllerToAttach` null)
      (`self.SetActorTickEnabled` false)
      (set `self.autoMovement` false)
      (set `self.ChangeValueMov` 0.0))
    (else
      (set `self.TickDeltaSeconds` DeltaSeconds)
      ;[1 1 1] Toolbox moving
      (set `self.OldBoxPosition` _x)
      (`SceneComponent.K2_SetWorldLocation` (`self.ControllerScene`) (`SceneComponent.K2_GetComponentLocation` (`self.ControllerToAttach`)) false false)
      (`SceneComponent.K2_SetRelativeLocation` _sm_toolbox_shelf (`KismetMathLibrary.MakeVector` (`KismetMathLibrary.FClamp` _x (`self.MaxPosition`) (`self.MinPosition`)) (.y (`SceneComponent.RelativeLocation` _sm_toolbox_shelf)) (.z (`SceneComponent.RelativeLocation` _sm_toolbox_shelf))) false false))))

(fn `UserConstructionScript`)