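; Right-hand cupboard door that a controller component can grab, swing on its hinge within set yaw limits, and release.
; Pickup enables Tick, which turns the door toward the controller's position through a look-at yaw and records the last angle.
; Drop, or straying too far from the handle sphere, releases it.
; A fast release keeps the door swinging with decaying angular velocity until Tick switches off.
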(event `/Game/VirtualRealityBP/Blueprints/PickupActorInterface.Pickup`
  (params (AttachTo :type "SceneComponent Object Reference"))
  ;[1 1 1] Pickup event
  (`/Engine/EditorBlueprintResources/StandardMacros.IsValid` AttachTo
    (:`Is Valid`
      (`/Engine/EditorBlueprintResources/StandardMacros.IsValid` (`self.ControllerToAttach`)
        (:`Is Not Valid`
          (if (`self.AutoMovement`)
            (set `self.AutoMovement` false)
            (set `self.AutoMovementValue` 0.0)
            (set `self.OldPos` 0.0)
            (set `self.TickDeltaSeconds` 0.0))
          (set `self.ControllerToAttach` AttachTo)
          (`self.SetActorTickEnabled` true))))))

(event `/Game/VirtualRealityBP/Blueprints/PickupActorInterface.Drop`
  (params (DeatacthFrom :type "SceneComponent Object Reference"))
  (bind _controllertoattach (`self.ControllerToAttach`))
  (bind _returnvalue (/ (- (`KismetMathLibrary.FClamp` (- (.yaw (`KismetMathLibrary.FindLookAtRotation` (`SceneComponent.RelativeLocation` (`self.ControllerScene`)) (`SceneComponent.RelativeLocation` (`self.Scene`)))) 90.0) (* (`self.MaxPos`) -1.0) (`self.MinPos`)) (`self.OldPos`)) (`self.TickDeltaSeconds`)))
  ;[1 1 1] Drop event
  (`/Engine/EditorBlueprintResources/StandardMacros.IsValid` DeatacthFrom
    (:`Is Valid`
      (`/Engine/EditorBlueprintResources/StandardMacros.IsValid` _controllertoattach
        (:`Is Valid`
          (if (== _controllertoattach DeatacthFrom)
            (if (or (> _returnvalue 25.0) (< _returnvalue -25.0)) :!label _label
              (set `self.AutoMovement` true)
              (set `self.AutoMovementValue` _returnvalue)
              (set `self.ControllerToAttach` null)
              (set `self.ChangeValue` 0.0)
              (else
                (set `self.ControllerToAttach` null)
                (`self.SetActorTickEnabled` false)))))))))

(event `self.ReceiveTick`
  (params (DeltaSeconds :type "Float (single-precision)"))
  (bind _controllerscene (`self.ControllerScene`))
  (bind _automovementvalue (`self.AutoMovementValue`))
  (bind _sm_toolbox_door_r (`self.SM_Toolbox_Door_R`))
  (bind _returnvalue (`SceneComponent.K2_GetComponentLocation` (`self.ControllerToAttach`)))
  (bind _returnvalue_2 (`KismetMathLibrary.FClamp` (- (.yaw (`KismetMathLibrary.FindLookAtRotation` (`SceneComponent.RelativeLocation` _controllerscene) (`SceneComponent.RelativeLocation` (`self.Scene`)))) 90.0) (* (`self.MaxPos`) -1.0) (`self.MinPos`)))
  (if (`self.AutoMovement`)
    (bind _output_get (set `self.ChangeValue` (- (`self.ChangeValue`) (/ _automovementvalue 100.0))))
    (`SceneComponent.K2_SetRelativeRotation` _sm_toolbox_door_r (`KismetMathLibrary.MakeRotator` (.roll (`SceneComponent.RelativeRotation` _sm_toolbox_door_r)) (.pitch (`SceneComponent.RelativeRotation` _sm_toolbox_door_r)) (`KismetMathLibrary.FClamp` (- _returnvalue_2 _output_get) (* (`self.MaxPos`) -1.0) (`self.MinPos`))) false false)
    (bind _output_get_2 (set `self.AutoMovementValue` (/ _automovementvalue 1.05)))
    (if (`KismetMathLibrary.NearlyEqual_FloatFloat` _output_get_2 0.0 1.0)
      (set `self.AutoMovement` false)
      (set `self.AutoMovementValue` 0.0)
      (set `self.ChangeValue` 0.0)
      (set `self.TickDeltaSeconds` 0.0)
      (set `self.OldPos` 0.0)
      (`self.SetActorTickEnabled` false))
    (else
      (set `self.OldPos` _returnvalue_2)
      (set `self.TickDeltaSeconds` DeltaSeconds)
      (`SceneComponent.K2_SetWorldLocation` _controllerscene _returnvalue false false)
      (if (> (`KismetMathLibrary.Vector_Distance` _returnvalue (`SceneComponent.K2_GetComponentLocation` (`self.Sphere`))) 30.0)
        (goto _label)
        (else
          (`SceneComponent.K2_SetRelativeRotation` (`self.SM_Toolbox_Door_R`) (`KismetMathLibrary.MakeRotator` (.roll (`SceneComponent.RelativeRotation` (`self.SM_Toolbox_Door_R`))) (.pitch (`SceneComponent.RelativeRotation` (`self.SM_Toolbox_Door_R`))) _returnvalue_2) false false))))))

(fn `UserConstructionScript`)