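; VR table actor that the player resizes and repositions using the right motion controller.
; Overlapping ScaleTrigger tints the panel through a material parameter collection and rumbles; a trigger press there enters scale mode.
; Two further presses capture probe corners, shown as debug spheres, then TransformTable centers and scales the mesh against its P1/P2 markers.
; It also moves the "MLS"-tagged actor just above the new center; rotation code is unconnected.
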(event `self.ReceiveBeginPlay`
  (`KismetSystemLibrary.Delay` 1.0)
  ;[1 1 1] Get ref on motion controller pawn
  (bind _outactors (`GameplayStatics.GetAllActorsOfClass` "/Game/VirtualRealityBP/Blueprints/MotionControllerPawn.MotionControllerPawn_C"))
  (set `self.MCPawnRef` (`|GetArrayItem` _outactors))
  (bind _outactors_2 (`GameplayStatics.GetAllActorsWithTag` "MLS"))
  (bind _output (`|GetArrayItem` _outactors_2))
  (`/Engine/EditorBlueprintResources/StandardMacros.IsValid` _output
    (:`Is Valid`
      (set `self.MLS_REF` _output))))

(event `Key|MotionController_Right_Trigger` :consume false :overrideparent false
  (params (Key :type "Key Structure"))
  (:`Released`
    ;[1 1 1] Subscribing to inputs
    (set `self.TakeInput` true :!label _label)))

(event `TRL`
  ;[1 1 1] Subscribing to inputs
  (goto _label))

(event `TRP`
  ;[1 1 1] Subscribing to inputs
  (`self.TriggerPress`))

(event `self.ReceiveTick`
  (params (DeltaSeconds :type "Float (single-precision)"))
  (bind _mcpawnref (`self.MCPawnRef`))
  (bind _rightcontroller (`/Game/VirtualRealityBP/Blueprints/MotionControllerPawn.RightController` _mcpawnref))
  (bind _returnvalue (`SceneComponent.K2_GetComponentLocation` (`/Game/VirtualRealityBP/Blueprints/BP_MotionController.Probe` (`/Game/VirtualRealityBP/Blueprints/MotionControllerPawn.RightController` (`self.MCPawnRef`)))))
  (if (`self.ScaleMode`)
    ;[1 1 1] Drawing_Points
    (`KismetSystemLibrary.DrawDebugSphere` (`self.Vector1`) 5.0 12 (struct :`R` 0.491696 :`G` 1.0 :`A` 1.0) 0.1)
    (`KismetSystemLibrary.DrawDebugSphere` (`self.Vector2`) 5.0 12 (struct :`R` 0.023903 :`B` 1.0 :`A` 1.0) 0.1)
    (`KismetSystemLibrary.DrawDebugSphere` (`SceneComponent.K2_GetComponentLocation` (`self.P2`)) 5.0 12 (struct :`A` 1.0) 0.1)
    (`KismetSystemLibrary.DrawDebugSphere` (`SceneComponent.K2_GetComponentLocation` (`self.P1`)) 5.0 12 (struct :`A` 1.0) 0.1)
    (if (`self.Point1`)
      (`KismetSystemLibrary.DrawDebugSphere` _returnvalue 1.0 12 (struct :`R` 0.023903 :`B` 1.0 :`A` 1.0) 0.1)
      (else
        (`KismetSystemLibrary.DrawDebugSphere` _returnvalue 1.0 12 (struct :`R` 0.491696 :`G` 1.0 :`A` 1.0) 0.1)))
    (else
      (`/Engine/EditorBlueprintResources/StandardMacros.IsValid` _mcpawnref
        (:`Is Valid`
          ;[1 1 1] CheckingOverlap
          (if (`PrimitiveComponent.IsOverlappingComponent` (`self.ScaleTrigger`) (`/Game/VirtualRealityBP/Blueprints/BP_MotionController.GrabSphere` _rightcontroller))
            (set `self.Overlaping` true)
            (`KismetMaterialLibrary.SetVectorParameterValue` "/Game/VirtualReality/Materials/TeleportMCP.TeleportMCP" "TablePanelColor" (make `LinearColor` 1.0 0.0 0.0 0.3))
            ;[1 1 1] Rumble
            (`/Engine/EditorBlueprintResources/StandardMacros.DoOnce` false :!label _label_2
              (:`Completed`
                (`/Game/VirtualRealityBP/Blueprints/BP_MotionController.RumbleController` _rightcontroller 0.2)
                (`KismetSystemLibrary.Delay` 0.5)
                (goto _label_2 :!via `Reset`)))
            (else
              (set `self.Overlaping` false)
              (`KismetMaterialLibrary.SetVectorParameterValue` "/Game/VirtualReality/Materials/TeleportMCP.TeleportMCP" "TablePanelColor" (make `LinearColor` 1.0 1.0 1.0 1.0)))))))))

(event `TriggerPress`
  (bind _returnvalue (`SceneComponent.K2_GetComponentLocation` (`/Game/VirtualRealityBP/Blueprints/BP_MotionController.Probe` (`/Game/VirtualRealityBP/Blueprints/MotionControllerPawn.RightController` (`self.MCPawnRef`)))))
  ;[1 1 1] Input sequence
  (if (`self.TakeInput`) :!label _label_3
    (if (`self.ScaleMode`)
      (if (`self.Point1`)
        (set `self.Vector2` (`KismetMathLibrary.MakeVector` (.x _returnvalue) (.y _returnvalue) (.z (stale _output_get))))
        (set `self.Point1` false)
        (set `self.ScaleMode` false)
        (`self.TransformTable`)
        (else
          (bind _output_get (set `self.Vector1` _returnvalue))
          (set `self.Point1` true)))
      (elif (`self.Overlaping`)
        (set `self.ScaleMode` true)
        (set `self.Point1` false)))))

(event `Key|MotionController_Right_Trigger` :consume false :overrideparent false
  (params (Key :type "Key Structure"))
  (:`Pressed`
    (goto _label_3)))

(event `TransformTable`
  (bind _vector1 (`self.Vector1`))
  (bind _vector2 (`self.Vector2`))
  (bind _sm_table (`self.SM_Table`))
  (bind (_returnvalue_x _returnvalue_y _returnvalue_z) (`KismetMathLibrary.BreakVector` (`SceneComponent.K2_GetComponentLocation` _sm_table)))
  (bind (_returnvalue_x_2 _returnvalue_y_2) (`KismetMathLibrary.BreakVector` (`SceneComponent.K2_GetComponentLocation` (`self.P2`))))
  (bind (_returnvalue_x_3 _returnvalue_y_3) (`KismetMathLibrary.BreakVector` (`SceneComponent.K2_GetComponentLocation` (`self.P1`))))
  (bind (_returnvalue_x_4 _returnvalue_y_4 _returnvalue_z_2) (`KismetMathLibrary.BreakVector` (`SceneComponent.K2_GetComponentLocation` (`self.SM_Table`))))
  (bind (_returnvalue_x_5 _returnvalue_y_5 _returnvalue_z_3) (`KismetMathLibrary.BreakVector` (`SceneComponent.K2_GetComponentLocation` (`self.P1`))))
  (bind _x (.x (`KismetMathLibrary.VLerp` _vector1 _vector2 0.5)))
  (bind _y (.y (`KismetMathLibrary.VLerp` _vector1 _vector2 0.5)))
  ;[1 1 1] Transfrom
  (set `self.MLS_Spot` (`KismetMathLibrary.MakeVector` _x _y (+ (.z (`KismetMathLibrary.VLerp` _vector1 _vector2 0.5)) 7.0)))
  (`SceneComponent.K2_SetWorldLocationAndRotation` :`self` _sm_table :`NewLocation` (`KismetMathLibrary.MakeVector` _x _y _returnvalue_z))
  (`SceneComponent.SetWorldScale3D` _sm_table (`KismetMathLibrary.MakeVector` (`KismetMathLibrary.Abs` (* (.x (`SceneComponent.K2_GetComponentScale` _sm_table)) (/ (- (.x _vector1) (.x _vector2)) (- _returnvalue_x_3 _returnvalue_x_2)))) (`KismetMathLibrary.Abs` (* (.y (`SceneComponent.K2_GetComponentScale` _sm_table)) (/ (- (.y _vector1) (.y _vector2)) (- _returnvalue_y_3 _returnvalue_y_2)))) (`KismetMathLibrary.Abs` (* (.z (`SceneComponent.K2_GetComponentScale` _sm_table)) (/ (- _returnvalue_z_2 (.z _vector1)) (- _returnvalue_z_2 _returnvalue_z_3))))))
  (`self.K2_SetActorLocation` (`self.MLS_REF`) (`self.MLS_Spot`) false false))

(fn `UserConstructionScript`)