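; Actor that receives inverted pendulum state, apparently over UDP, and passes caret position and pendulum angle to other objects.
; Each Tick it reads two floats from GetData and sends them to SendToImplementationObject through DeliverDataMessage.
; In parallel, the FakeData timeline starts at BeginPlay and streams simulated values to SendFakeData through the same message, with a FlipFlop alternating reverse and forward playback in an endless loop.
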(event `self.ReceiveTick`
  (params (DeltaSeconds :type "Float (single-precision)"))
  (bind _returnvalue (`self.GetData`))
  (bind (_float1 _float2) (break `UDPData` _returnvalue))
  (message `/Game/Blueprints/InvpDDeliverInterface.DeliverData` (`self.SendToImplementationObject`) _float1 _float2))

(event `self.ReceiveBeginPlay`
  (bind (_direction _kareta _pendulum) (`Timeline|FakeData` :!label _label)
    (:`Update`
      (message `/Game/Blueprints/InvpDDeliverInterface.DeliverData` (`self.SendFakeData`) _kareta _pendulum))
    (:`Finished`
      (`self.SendMore`))))

(event `SendMore`
  (`/Engine/EditorBlueprintResources/StandardMacros.FlipFlop`
    (:`A`
      (goto _label :!via `Reverse`))
    (:`B`
      (goto _label :!via `PlayFromStart`))))

(fn `UserConstructionScript`)