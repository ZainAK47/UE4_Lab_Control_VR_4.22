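; Feature manager for fitting a VR table to two points marked with the left controller.
; A trigger press while overlapping enters scale mode, and the next two presses record grab-sphere positions.
; TransformTable centers the table between them and scales X/Y by their distance relative to its P1–P2 span, keeping Z.
; Input binding, overlap detection and feedback are disconnected, so nothing here starts the flow.
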(event `self.ReceiveBeginPlay`)

(event `TRP`
  (`self.TriggerPress`))

(event `TRL`
  (set `self.TakeInput` true))

(event `self.ReceiveTick`
  (params (DeltaSeconds :type "Float (single-precision)")))

(event `TriggerPress`
  (bind _returnvalue (`SceneComponent.K2_GetComponentLocation` (`/Game/VirtualRealityBP/Blueprints/BP_MotionController.GrabSphere` (`/Game/VirtualRealityBP/Blueprints/MotionControllerPawn.LeftController` (`self.MCPawnRef`)))))
  (if (`self.TakeInput`)
    (if (`self.ScaleMode`)
      (if (`self.Point1`)
        (set `self.Vector2` _returnvalue)
        (set `self.ScaleMode` false)
        (set `self.Point1` false)
        (`self.TransformTable`)
        (else
          (set `self.Vector1` _returnvalue)
          (set `self.Point1` true)))
      (elif (`self.Overlaping`)
        (set `self.ScaleMode` true)
        (set `self.Point1` false)))))

(event `TransformTable`
  (bind _tableref (`self.TableRef`))
  (bind _vector1 (`self.Vector1`))
  (bind _vector2 (`self.Vector2`))
  (bind _sm_table (`/Game/Blueprints/Table_BP.SM_Table` (`self.TableRef`)))
  (bind (_returnvalue_x _returnvalue_y _returnvalue_z) (`KismetMathLibrary.BreakVector` (`SceneComponent.K2_GetComponentLocation` _sm_table)))
  (bind (_returnvalue_x_2 _returnvalue_y_2 _returnvalue_z_2) (`KismetMathLibrary.BreakVector` (`SceneComponent.K2_GetComponentScale` _sm_table)))
  (bind (_returnvalue_x_3 _returnvalue_y_3) (`KismetMathLibrary.BreakVector` (* (`SceneComponent.K2_GetComponentScale` _sm_table) (/ (`KismetMathLibrary.Vector_Distance` _vector1 _vector2) (`KismetMathLibrary.Vector_Distance` (`SceneComponent.K2_GetComponentLocation` (`/Game/Blueprints/Table_BP.P1` _tableref)) (`SceneComponent.K2_GetComponentLocation` (`/Game/Blueprints/Table_BP.P2` _tableref)))))))
  (`SceneComponent.K2_SetWorldLocationAndRotation` :`self` _sm_table :`NewLocation` (`KismetMathLibrary.MakeVector` (.x (`KismetMathLibrary.VLerp` _vector1 _vector2 0.5)) (.y (`KismetMathLibrary.VLerp` _vector1 _vector2 0.5)) _returnvalue_z))
  (`SceneComponent.SetWorldScale3D` _sm_table (`KismetMathLibrary.MakeVector` _returnvalue_x_3 _returnvalue_y_3 _returnvalue_z_2)))

(fn `UserConstructionScript`)