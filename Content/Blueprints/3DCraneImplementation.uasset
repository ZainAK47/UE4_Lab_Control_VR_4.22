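; 3D crane actor that visualizes crane motion from position and angle values passed to its DeliverData event.
; X slides the black frame along local Y, while Y slides the transparent part along local X from a default offset set at BeginPlay.
; Alpha and Beta set the weight's roll and pitch to show its swing.
; Transforms are applied directly without sweep, and the Blueprint computes no physics itself.
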(event `self.ReceiveBeginPlay`
  (set `self.TransPartDefLoc` -35.0))

(event `/Game/Blueprints/3DCraneDDeliverInterface.DeliverData`
  (params (x :type "Float (single-precision)") (y :type "Float (single-precision)") (z :type "Float (single-precision)") (alpha :type "Float (single-precision)") (beta :type "Float (single-precision)"))
  (`SceneComponent.K2_SetRelativeLocation` (`self.Blackframev4`) (`KismetMathLibrary.MakeVector` 0.0 x) false false)
  (`SceneComponent.K2_SetRelativeLocation` (`self.Transparentpart`) (`KismetMathLibrary.MakeVector` (+ (`self.TransPartDefLoc`) y)) false false)
  (`SceneComponent.K2_SetRelativeRotation` (`self.weightv1`) (`KismetMathLibrary.MakeRotator` alpha beta) false false))

(fn `UserConstructionScript`)