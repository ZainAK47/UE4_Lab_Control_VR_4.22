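; VR table that the player resizes and repositions by marking three points with the right motion controller.
; Trigger presses inside ScaleTrigger, cued by panel color and rumble, start scale mode, then record probe positions flattened to the first point's height.
; TransformTable treats the longest point pair as the diagonal, deriving center, yaw and clamped footprint scale.
; It also adjusts height and legs and moves the PutOnTheTable actor to the center.
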(event `self.ReceiveBeginPlay`
  (`KismetSystemLibrary.Delay` 1.0)
  ;[1 1 1] Get ref on motion controller pawn
  (bind _outactors (`GameplayStatics.GetAllActorsOfClass` "/Game/VirtualRealityBP/Blueprints/MotionControllerPawn.MotionControllerPawn_C"))
  (set `self.MCPawnRef` (`|GetArrayItem` _outactors)))

(event `self.ReceiveTick`
  (params (DeltaSeconds :type "Float (single-precision)"))
  (bind _returnvalue (`SceneComponent.K2_GetComponentLocation` (`/Game/VirtualRealityBP/Blueprints/BP_MotionController.Probe` (`/Game/VirtualRealityBP/Blueprints/MotionControllerPawn.RightController` (`self.MCPawnRef`)))))
  (if (`self.ScaleMode`)
    ;[1 1 1] Drawing_Points
    (`KismetSystemLibrary.DrawDebugSphere` (`self.VPoint1`) 5.0 12 (struct :`R` 0.491696 :`G` 1.0 :`A` 1.0) 0.1)
    (`KismetSystemLibrary.DrawDebugSphere` (`self.VPoint2`) 5.0 12 (struct :`R` 0.023903 :`B` 1.0 :`A` 1.0) 0.1)
    (`KismetSystemLibrary.DrawDebugSphere` (`self.VPoint3`) 5.0 12 (struct :`R` 1.0 :`A` 1.0) 0.1)
    (`KismetSystemLibrary.DrawDebugSphere` (`SceneComponent.K2_GetComponentLocation` (`self.P2`)) 5.0 12 (struct :`A` 1.0) 0.1)
    (`KismetSystemLibrary.DrawDebugSphere` (`SceneComponent.K2_GetComponentLocation` (`self.P1`)) 5.0 12 (struct :`A` 1.0) 0.1)
    (`KismetSystemLibrary.DrawDebugSphere` (`SceneComponent.K2_GetComponentLocation` (`self.P3`)) 5.0 12 (struct :`A` 1.0) 0.1)
    (if true
      (`KismetSystemLibrary.DrawDebugSphere` _returnvalue 1.0 12 (struct :`R` 0.023903 :`B` 1.0 :`A` 1.0) 0.1)
      (else
        (`KismetSystemLibrary.DrawDebugSphere` _returnvalue 1.0 12 (struct :`R` 0.491696 :`G` 1.0 :`A` 1.0) 0.1)))))

(event `self.ScaleTrigger.OnComponentBeginOverlap`
  (params (OverlappedComponent :type "PrimitiveComponent Object Reference") (OtherActor :type "Actor Object Reference") (OtherComp :type "PrimitiveComponent Object Reference") (OtherBodyIndex :type Integer) (bFromSweep :type Boolean) (SweepResult :type "HitResult Structure (by ref)"))
  (bind _mcpawnref (`self.MCPawnRef`))
  (bind _rightcontroller (`/Game/VirtualRealityBP/Blueprints/MotionControllerPawn.RightController` _mcpawnref))
  ;[1 1 1] CheckingOverlap
  (`/Engine/EditorBlueprintResources/StandardMacros.IsValid` _mcpawnref
    (:`Is Valid`
      (if (== OtherComp (`/Game/VirtualRealityBP/Blueprints/BP_MotionController.GrabSphere` _rightcontroller))
        (set `self.Overlaping` true)
        (`KismetMaterialLibrary.SetVectorParameterValue` "/Game/VirtualReality/Materials/TeleportMCP.TeleportMCP" "TablePanelColor" (make `LinearColor` 1.0 0.0 0.0 0.3))
        (`/Engine/EditorBlueprintResources/StandardMacros.DoOnce` false
          (:`Completed`
            (if (`self.Overlaping`) :!label _label
              (if (not (`self.ScaleMode`))
                (`/Game/VirtualRealityBP/Blueprints/BP_MotionController.RumbleController` _rightcontroller 0.2)))
            (`KismetSystemLibrary.Delay` 0.5)
            (goto _label)))))))

(event `self.ScaleTrigger.OnComponentEndOverlap`
  (params (OverlappedComponent :type "PrimitiveComponent Object Reference") (OtherActor :type "Actor Object Reference") (OtherComp :type "PrimitiveComponent Object Reference") (OtherBodyIndex :type Integer))
  (bind _mcpawnref (`self.MCPawnRef`))
  ;[1 1 1] CheckingOverlap
  (`/Engine/EditorBlueprintResources/StandardMacros.IsValid` _mcpawnref
    (:`Is Valid`
      (if (== OtherComp (`/Game/VirtualRealityBP/Blueprints/BP_MotionController.GrabSphere` (`/Game/VirtualRealityBP/Blueprints/MotionControllerPawn.RightController` _mcpawnref)))
        (set `self.Overlaping` false)
        (`KismetMaterialLibrary.SetVectorParameterValue` "/Game/VirtualReality/Materials/TeleportMCP.TeleportMCP" "TablePanelColor" (make `LinearColor` 1.0 1.0 1.0 1.0))))))

(event `Key|MotionController_Right_Trigger` :consume false :overrideparent false
  (params (Key :type "Key Structure"))
  (bind _returnvalue (`SceneComponent.K2_GetComponentLocation` (`/Game/VirtualRealityBP/Blueprints/BP_MotionController.Probe` (`/Game/VirtualRealityBP/Blueprints/MotionControllerPawn.RightController` (`self.MCPawnRef`)))))
  (bind _x (.x _returnvalue))
  (bind _y (.y _returnvalue))
  ;[1 1 1] Input sequence
  (:`Pressed`
    (if (`self.TakeInput`)
      (if (`self.ScaleMode`)
        (if (`self.P1set`)
          (if (`self.P2set`)
            (set `self.VPoint3` (`KismetMathLibrary.MakeVector` _x _y (.z (stale _output_get))))
            (set `self.ScaleMode` false)
            (`self.TransformTable`)
            (set `self.P1set` false)
            (set `self.P2set` false)
            (else
              (set `self.VPoint2` (`KismetMathLibrary.MakeVector` _x _y (.z (stale _output_get))))
              (set `self.P2set` true)))
          (else
            (bind _output_get (set `self.VPoint1` _returnvalue))
            (set `self.P1set` true)))
        (`/Game/VirtualRealityBP/Blueprints/BP_MotionController.RumbleController` (`/Game/VirtualRealityBP/Blueprints/MotionControllerPawn.RightController` (`self.MCPawnRef`)) 0.1)
        (elif (`self.Overlaping`)
          (set `self.ScaleMode` true)
          (set `self.P1set` false)
          (set `self.P2set` false))))))

(event `Key|MotionController_Right_Trigger` :consume false :overrideparent false
  (params (Key :type "Key Structure"))
  ;[1 1 1] Input sequence
  (:`Released`
    (set `self.TakeInput` true)))

(event `TransformTable`
  (bind _vpoint1 (`self.VPoint1`))
  (bind _vpoint2 (`self.VPoint2`))
  (bind _sm_table (`self.SM_Table`))
  (bind _tabledimensions (`self.TableDimensions`))
  (bind _sm_table_leg (`self.SM_Table_Leg`))
  (bind _vpoint3 (`self.VPoint3`))
  (bind (_returnvalue_x _returnvalue_y _returnvalue_z) (`KismetMathLibrary.BreakVector` (`SceneComponent.K2_GetComponentLocation` _sm_table)))
  (bind (_returnvalue_x_2 _returnvalue_y_2 _returnvalue_z_2) (`KismetMathLibrary.BreakVector` (`SceneComponent.K2_GetComponentLocation` (`self.SM_Table`))))
  (bind (_returnvalue_x_3 _returnvalue_y_3 _returnvalue_z_3) (`KismetMathLibrary.BreakVector` (`SceneComponent.K2_GetComponentLocation` (`self.P1`))))
  (bind _returnvalue (`SceneComponent.K2_GetComponentLocation` (`self.P2`)))
  (bind _returnvalue_2 (`KismetMathLibrary.Abs` (* (.z (`SceneComponent.K2_GetComponentScale` _sm_table)) (/ (- _returnvalue_z_2 (.z (`self.VPoint1`))) (- _returnvalue_z_2 _returnvalue_z_3)))))
  ;[1 1 1] Transfrom
  (bind _arrout (`self.Sorter` (`|MakeArray` (`KismetMathLibrary.Vector_Distance` _vpoint1 _vpoint2) (`KismetMathLibrary.Vector_Distance` _vpoint2 _vpoint3) (`KismetMathLibrary.Vector_Distance` _vpoint1 _vpoint3))))
  (bind _output_get (set `self.TableDimensions` _arrout))
  (bind (_center _newrotation) (`self.GetDiag` (`|MakeArray` _vpoint1 _vpoint2 _vpoint3) (`|GetArrayItem` _output_get 2)))
  (bind _output_get_2 (set `self.TableCenter` _center))
  (set `self.NEwTableRotation` _newrotation)
  (bind _x (.x _output_get_2))
  (bind _y (.y _output_get_2))
  (set `self.TableSpot` (`KismetMathLibrary.MakeVector` _x _y (+ (.z _output_get_2) 0.0)))
  (bind _returnvalue_3 (`KismetMathLibrary.MakeVector` _x _y _returnvalue_z))
  (`SceneComponent.K2_SetWorldTransform` _sm_table (`KismetMathLibrary.MakeTransform` _returnvalue_3 (`self.NEwTableRotation`) (`KismetMathLibrary.MakeVector` (`KismetMathLibrary.FClamp` (`KismetMathLibrary.Abs` (* (.x (`SceneComponent.K2_GetComponentScale` _sm_table)) (/ (`|GetArrayItem` _tabledimensions) (`KismetMathLibrary.Vector_Distance` _returnvalue (`SceneComponent.K2_GetComponentLocation` (`self.P3`)))))) 0.9 2.0) (`KismetMathLibrary.FClamp` (`KismetMathLibrary.Abs` (* (.y (`SceneComponent.K2_GetComponentScale` _sm_table)) (/ (`|GetArrayItem` _tabledimensions 1) (`KismetMathLibrary.Vector_Distance` (`SceneComponent.K2_GetComponentLocation` (`self.P1`)) _returnvalue)))) 0.4 2.0) _returnvalue_2)) false false)
  (`SceneComponent.K2_SetWorldTransform` _sm_table_leg (`KismetMathLibrary.MakeTransform` _returnvalue_3 (struct) (`KismetMathLibrary.MakeVector` (.x (`SceneComponent.K2_GetComponentScale` _sm_table_leg)) (.y (`SceneComponent.K2_GetComponentScale` _sm_table_leg)) _returnvalue_2)) false false)
  (`self.K2_SetActorTransform` (`self.PutOnTheTable`) (`KismetMathLibrary.MakeTransform` (`self.TableSpot`) (`self.NEwTableRotation`)) false false))

(fn `GetDiag`
  (params (PointsIn :type "Array of Vector Structure") (DiagLength :type "Float (double-precision)"))
  (returns (Center :type "Vector Structure") (NewRotation :type "Rotator Structure"))
  (locals (Temp :type "Vector Structure") (Rotation :type "Rotator Structure") (D1 :type "Vector Structure") (D2 :type "Vector Structure"))
  (bind _d1 (`local.D1`))
  (bind _d2 (`local.D2`))
  (for _array_element PointsIn :!label _label
    (for _array_element_2 PointsIn
      (if (== (`KismetMathLibrary.Vector_Distance` _array_element _array_element_2) DiagLength)
        (set `local.D1` _array_element_2)
        (set `local.D2` _array_element)
        (bind _output_get (set `local.Temp` (`KismetMathLibrary.VLerp` _array_element_2 _array_element 0.5)))
        (goto _label :!via `Break`))))
  (for _array_element_3 PointsIn
    (if (and (!= _array_element_3 _d1) (!= _array_element_3 _d2))
      (if (< (`KismetMathLibrary.Vector_Distance` _array_element_3 _d1) (`KismetMathLibrary.Vector_Distance` _array_element_3 _d2))
        (bind _output_get_2 (set `local.Rotation` (`KismetMathLibrary.FindLookAtRotation` _array_element_3 _d1)))
        (break)
        (else
          (set `local.Rotation` (`KismetMathLibrary.FindLookAtRotation` _array_element_3 _d2))
          (break)))))
  (return _output_get _output_get_2))

(fn `Sorter`
  (params (ArrIn :type "Array of Float (double-precision)"))
  (returns (ArrOut :type "Array of Float (double-precision)"))
  (locals (Temp :type "Float (double-precision)"))
  (for (_array_element _array_index) ArrIn
    (for (_array_element_2 _array_index_2) ArrIn
      (if (<= _array_element _array_element_2)
        (bind _output_get (set `local.Temp` _array_element))
        (`KismetArrayLibrary.Array_Set` ArrIn _array_index _array_element_2)
        (`KismetArrayLibrary.Array_Set` ArrIn _array_index_2 _output_get))))
  (return ArrIn))

(fn `UserConstructionScript`)