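; BP_Hider2 is an actor in the coupled tanks project that feeds a plane's position and orientation to a material, apparently for clip-plane hiding.
; Its construction script writes the Plane component's world location and up vector into the "pos" and "normal" vector parameters.
; Tick calls Hider2Function every frame, whose body is not defined in this graph.
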(event `self.ReceiveTick`
  (params (DeltaSeconds :type "Float (single-precision)"))
  (`/Game/CoupledTanksProject/Blueprints/BP_Interface_Hider.Hider2_Function`))

(fn `UserConstructionScript`
  (bind _plane (`self.Plane`))
  (`KismetMaterialLibrary.SetVectorParameterValue` null "pos" (`KismetMathLibrary.Conv_VectorToLinearColor` (`SceneComponent.K2_GetComponentLocation` _plane)))
  (`KismetMaterialLibrary.SetVectorParameterValue` null "normal" (`KismetMathLibrary.Conv_VectorToLinearColor` (`SceneComponent.GetUpVector` _plane))))