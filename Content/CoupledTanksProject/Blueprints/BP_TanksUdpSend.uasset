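; BP_TanksUdpSend is an actor that streams coupled-tanks state over UDP to a subnet broadcast address.
; BeginPlay starts the UDP sender socket.
; Tick, throttled by a short Delay, packs three tank H values from CustomViveMotionController and two sphere scales, printed as KP and KI, into one float packet.
; A separate SendUDPData event sends only the three tank values.
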(event `self.ReceiveTick`
  (params (DeltaSeconds :type "Float (single-precision)"))
  (bind _spherescaletobesent_sphere1 (`self.SphereScaleToBeSent_Sphere1`))
  (bind _customvivemotioncontroller (`self.CustomViveMotionController`))
  (bind _spherescaletobesent_sphere2 (`self.SphereScaleToBeSent_Sphere2`))
  (`KismetSystemLibrary.Delay` 0.05)
  (`self.UDPSendArray` (make `UDPData` (`/Game/CoupledTanksProject/Blueprints/BP_Tanks_CustomViveMotionController.tank1H` _customvivemotioncontroller) (`/Game/CoupledTanksProject/Blueprints/BP_Tanks_CustomViveMotionController.tank2H` _customvivemotioncontroller) (`/Game/CoupledTanksProject/Blueprints/BP_Tanks_CustomViveMotionController.tank3H` _customvivemotioncontroller) _spherescaletobesent_sphere1 _spherescaletobesent_sphere2))
  (`KismetSystemLibrary.PrintString` (`KismetStringLibrary.Concat_StrStr` "                                                                                                        KP = " (`KismetStringLibrary.Conv_DoubleToString` _spherescaletobesent_sphere1)) true true (struct :`G` 0.66 :`B` 1.0 :`A` 1.0) 0.3)
  (`KismetSystemLibrary.PrintString` (`KismetStringLibrary.Concat_StrStr` "                                                                                                        KI = " (`KismetStringLibrary.Conv_DoubleToString` _spherescaletobesent_sphere2)) true true (struct :`G` 0.66 :`B` 1.0 :`A` 1.0) 0.3))

(event `self.ReceiveBeginPlay`
  (bind _returnvalue (`self.StartUDPSender` "sock2" "192.168.11.255" 9933))
  (set `self.UDPSender started` _returnvalue))

(event `Send UDP Data`
  (bind _customvivemotioncontroller (`self.CustomViveMotionController`))
  (`self.UDPSendArray` (make `UDPData` (`/Game/CoupledTanksProject/Blueprints/BP_Tanks_CustomViveMotionController.tank1H` _customvivemotioncontroller) (`/Game/CoupledTanksProject/Blueprints/BP_Tanks_CustomViveMotionController.tank2H` _customvivemotioncontroller) (`/Game/CoupledTanksProject/Blueprints/BP_Tanks_CustomViveMotionController.tank3H` _customvivemotioncontroller))))

(fn `UserConstructionScript`)