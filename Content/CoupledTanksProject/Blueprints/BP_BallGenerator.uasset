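; BP_BallGenerator is a scene component that supplies throwable balls on demand.
; GenerateBall spawns a scaled-down ThrowableBall at the component's world location and rotation, stores it as CurrentBall and attaches it to itself, keeping world transforms.
; ReleaseBall detaches the stored ball's static mesh and turns on physics simulation, letting it move freely.
; Both functions rely on external callers, as BeginPlay and Tick are empty.
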(fn `GenerateBall`
  (bind _returnvalue (`|SpawnActorFromClass` "/Game/CoupledTanksProject/Blueprints/ThrowableBall.ThrowableBall_C" (`KismetMathLibrary.MakeTransform` (.location (`self.K2_GetComponentToWorld`)) (.rotation (`self.K2_GetComponentToWorld`)) (0.05 0.05 0.05)) "Undefined" "OverrideRootScale" null null))
  (bind _output_get (set `self.CurrentBall` _returnvalue))
  (`Actor.K2_AttachToComponent` _output_get self "None" "KeepWorld" "KeepWorld" "KeepWorld" false))

(fn `ReleaseBall`
  (bind _staticmesh (`/Game/CoupledTanksProject/Blueprints/ThrowableBall.StaticMesh` (`self.CurrentBall`)))
  (`self.K2_DetachFromComponent` _staticmesh "KeepWorld" "KeepWorld" "KeepWorld" false)
  (`PrimitiveComponent.SetSimulatePhysics` _staticmesh true))