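; VR display socket that takes MovableWidget_BP panels released inside its Box and arranges them in a row.
; Overlapping a held panel binds to the MotionControllerPawn's grab release, which places and records it with its original scale; AddtoDisplayManualy bypasses the grab.
; ScaleWidgets drops duplicate or in-use entries, then rescales and repositions the rest between corner markers.
; Pulling an in-use panel out restores its scale and reflows the row.
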(event `self.Box.OnComponentEndOverlap`
  (params (OverlappedComponent :type "PrimitiveComponent Object Reference") (OtherActor :type "Actor Object Reference") (OtherComp :type "PrimitiveComponent Object Reference") (OtherBodyIndex :type Integer))
  (bind _arrayofwidgets (`self.ArrayOfWidgets`))
  (bind _asmotion_controller_pawn (cast `/Game/VirtualRealityBP/Blueprints/MotionControllerPawn` (`GameplayStatics.GetPlayerPawn` 0)))
  (bind _asmovable_widget_bp (cast `/Game/Blueprints/Widget_BP/MovableWidget_BP` OtherActor))
  (if (not (`/Game/Blueprints/Widget_BP/MovableWidget_BP.WasThrowed` _asmovable_widget_bp))
    (remove `/Game/VirtualRealityBP/Blueprints/MotionControllerPawn.Grab_Release` _asmotion_controller_pawn (delegate `Released`))
    (bind _asmovable_widget_bp_2 (cast `/Game/Blueprints/Widget_BP/MovableWidget_BP` OtherActor))
    (if (`/Game/Blueprints/Widget_BP/MovableWidget_BP.InUse` _asmovable_widget_bp_2)
      (for (_array_element _array_index) _arrayofwidgets
        (bind (_widget _leftdownpos _rightdownpos _leftuppos _rightuppos _downtoupdistance _lefttorightdistance _previousscale) (break `/Game/Blueprints/Widget_BP/ArrayOfWidgetsOnTheDisplay` _array_element))
        (if (== _widget OtherActor)
          (bind _output_get (set `self.RemovedWidget` _widget))
          (bind _output_get_2 (set `self.RemovedWidgetScale` _previousscale))
          (`KismetArrayLibrary.Array_Remove` _arrayofwidgets _array_index)
          (`self.SetActorScale3D` _output_get _output_get_2)
          (`self.K2_SetActorRelativeLocation` _output_get (0.0 0.0 0.0) false false)
          (set `self.RemovedWidget` null)
          (set `self.LastObject` null)
          (bind _arrayofwidgetsafterscaling (`self.ScaleWidgets`))
          (set `self.ArrayOfWidgets` _arrayofwidgetsafterscaling)
          (break))))))

(event `self.Box.OnComponentBeginOverlap`
  (params (OverlappedComponent :type "PrimitiveComponent Object Reference") (OtherActor :type "Actor Object Reference") (OtherComp :type "PrimitiveComponent Object Reference") (OtherBodyIndex :type Integer) (bFromSweep :type Boolean) (SweepResult :type "HitResult Structure (by ref)"))
  (bind _firsthand (`/Game/Blueprints/Widget_BP/MovableWidget_BP.FirstHand` (`self.MovableWidget`)))
  (bind _asmovable_widget_bp (cast `/Game/Blueprints/Widget_BP/MovableWidget_BP` OtherActor))
  (if (`/Game/Blueprints/Widget_BP/MovableWidget_BP.WasThrowed` _asmovable_widget_bp)
    _
    (elif (!= (`self.LastRemovedWidget`) _asmovable_widget_bp)
      (set `self.MovableWidget` _asmovable_widget_bp)
      (bind _asmotion_controller_pawn (cast `/Game/VirtualRealityBP/Blueprints/MotionControllerPawn` (`GameplayStatics.GetPlayerPawn` 0)))
      (`/Engine/EditorBlueprintResources/StandardMacros.IsValid` _firsthand
        (:`Is Valid`
          (set `self.ControllerSelectedToCheck` (`ActorComponent.GetOwner` _firsthand))
          (add `/Game/VirtualRealityBP/Blueprints/MotionControllerPawn.Grab_Release` _asmotion_controller_pawn (delegate `Released`)))))))

(event `Released`
  (params (ControllerReference :type "/Game/VirtualRealityBP/Blueprints/BP_MotionController Object Reference"))
  (bind _movablewidget (`self.MovableWidget`))
  (bind _movablewidget_2 (`self.MovableWidget`))
  (bind _padding (`self.Padding`))
  (bind _lefttorightdistcheck (`self.LeftToRightDistCheck`))
  (bind _downtoupdistcheck (`self.DownToUpDistCheck`))
  (bind _returnvalue (`SceneComponent.K2_GetComponentLocation` (`self.LeftDownPos`)))
  (bind _returnvalue_2 (`SceneComponent.K2_GetComponentLocation` (`/Game/Blueprints/Widget_BP/MovableWidget_BP.LeftDownPos_Wid` _movablewidget_2)))
  (bind _returnvalue_3 (`SceneComponent.K2_GetComponentLocation` (`/Game/Blueprints/Widget_BP/MovableWidget_BP.RightDownPos_Wid` _movablewidget_2)))
  (bind _returnvalue_4 (`SceneComponent.K2_GetComponentLocation` (`/Game/Blueprints/Widget_BP/MovableWidget_BP.LeftUpPos_Wid` _movablewidget_2)))
  (bind _returnvalue_5 (`KismetMathLibrary.Vector_Distance` _returnvalue_2 _returnvalue_3))
  (bind _returnvalue_6 (`KismetMathLibrary.Vector_Distance` _returnvalue_2 _returnvalue_4))
  (bind _asmotion_controller_pawn (cast `/Game/VirtualRealityBP/Blueprints/MotionControllerPawn` (`GameplayStatics.GetPlayerPawn` 0)))
  (if (== (`self.ControllerSelectedToCheck`) ControllerReference)
    (if (not (`/Game/Blueprints/Widget_BP/MovableWidget_BP.WasThrowed` (`self.MovableWidget`)))
      (remove `/Game/VirtualRealityBP/Blueprints/MotionControllerPawn.Grab_Release` _asmotion_controller_pawn (delegate `Released`))
      (`self.K2_SetActorLocationAndRotation` :`self` _movablewidget :`NewLocation` (`KismetMathLibrary.MakeVector` (/ (+ (.x (`SceneComponent.K2_GetComponentLocation` (`self.DefaultSceneRoot`))) (.x _returnvalue)) 2.0) (- (.y _returnvalue) (+ (+ (`self.LastAddedComponentDistRight`) _padding) (/ _returnvalue_5 2.0))) (+ (.z _returnvalue) (+ _padding (/ _returnvalue_6 2.0)))) :!label _label)
      (`KismetArrayLibrary.Array_Add` (`self.ArrayOfWidgets`) (make `/Game/Blueprints/Widget_BP/ArrayOfWidgetsOnTheDisplay` _movablewidget _returnvalue_2 _returnvalue_3 _returnvalue_4 (`SceneComponent.K2_GetComponentLocation` (`/Game/Blueprints/Widget_BP/MovableWidget_BP.RightUpPos_Wid` _movablewidget_2)) _returnvalue_6 _returnvalue_5 (`self.GetActorScale3D` _movablewidget_2)))
      (bind _arrayofwidgetsafterscaling (`self.ScaleWidgets`))
      (set `self.ArrayOfWidgets` _arrayofwidgetsafterscaling)
      (for _array_element (`self.ArrayOfWidgets`)
        (if (and (> _lefttorightdistcheck 0.0) (> _downtoupdistcheck 0.0))
          (bind (_widget _leftdownpos _rightdownpos _leftuppos _rightuppos _downtoupdistance _lefttorightdistance) (break `/Game/Blueprints/Widget_BP/ArrayOfWidgetsOnTheDisplay` _array_element))
          (if (not (and (== _lefttorightdistcheck _lefttorightdistance) (== _downtoupdistcheck _downtoupdistance)))
            (bind _arrayofwidgetsafterscaling_2 (`self.ScaleWidgets`))
            (set `self.ArrayOfWidgets` _arrayofwidgetsafterscaling_2)
            (break))
          (else
            (set `self.DownToUpDistCheck` _downtoupdistance)
            (set `self.LeftToRightDistCheck` _lefttorightdistance)))))))

(event `/Game/Blueprints/Widget_BP/WidgetControl_Interface.AddToDisplayManualy`
  (params (Actor :type "Actor Object Reference"))
  (bind _asmovable_widget_bp (cast `/Game/Blueprints/Widget_BP/MovableWidget_BP` Actor))
  (set `self.MovableWidget` _asmovable_widget_bp)
  (goto _label))

(fn `ScaleWidgets`
  (returns (ArrayOfWidgetsAfterScaling :type "Array of /Game/Blueprints/Widget_BP/ArrayOfWidgetsOnTheDisplay Structure"))
  (bind _arrayofwidgets (`self.ArrayOfWidgets`))
  (bind _padding (`self.Padding`))
  (bind _returnvalue (`SceneComponent.K2_GetComponentLocation` (`self.LeftDownPos`)))
  (set `self.ArrayOfLeft` 0.0)
  (set `self.ArrayOfUp` 0.0)
  (`KismetArrayLibrary.Array_Clear` (`self.WidgetArrayOnlyRefs`))
  (for (_array_element _array_index) _arrayofwidgets
    (bind _widget (break `/Game/Blueprints/Widget_BP/ArrayOfWidgetsOnTheDisplay` _array_element))
    (if (`KismetArrayLibrary.Array_Contains` (`self.WidgetArrayOnlyRefs`) _widget)
      (`KismetArrayLibrary.Array_RemoveItem` _arrayofwidgets _array_element :!label _label)
      (else
        (bind _asmovable_widget_bp (cast `/Game/Blueprints/Widget_BP/MovableWidget_BP` _widget)
          (:`then`
            (if (`/Game/Blueprints/Widget_BP/MovableWidget_BP.InUse` _asmovable_widget_bp)
              (goto _label)
              (else
                (set `self.ArrayOfLeft` (+ (+ 66.0 0.0) (`self.ArrayOfLeft`)))
                (set `self.ArrayOfUp` (+ (`self.ArrayOfUp`) (+ 0.0 50.0))))))
          (:`CastFailed`
            (goto _label))))))
  (`KismetArrayLibrary.Array_Clear` (`self.NewArrayOfWidgets`))
  (set `self.LastAddedComponentDistRight` 0.0)
  (for _array_element_2 (`self.ArrayOfWidgets`)
    (bind (_widget_2 _leftdownpos _rightdownpos _leftuppos _rightuppos _downtoupdistance _lefttorightdistance _previousscale) (break `/Game/Blueprints/Widget_BP/ArrayOfWidgetsOnTheDisplay` _array_element_2))
    (bind _returnvalue_2 (`KismetMathLibrary.Conv_IntToDouble` (+ _array_index 1)))
    (bind _returnvalue_3 (/ (`self.ArrayOfLeft`) _returnvalue_2))
    (bind _returnvalue_4 (* (/ (/ (`KismetMathLibrary.Vector_Distance` _returnvalue (`SceneComponent.K2_GetComponentLocation` (`self.RightDownPos`))) (+ _returnvalue_3 _padding)) _returnvalue_2) 1.0))
    (bind _returnvalue_5 (/ (`self.ArrayOfUp`) _returnvalue_2))
    (bind _returnvalue_6 (`KismetMathLibrary.FClamp` _returnvalue_4 _returnvalue_4 (/ (`KismetMathLibrary.Vector_Distance` (`SceneComponent.K2_GetComponentLocation` (`self.LeftUpPos`)) _returnvalue) (+ _returnvalue_5 _padding))))
    (`self.SetActorScale3D` _widget_2 (`KismetMathLibrary.MakeVector` 1.0 _returnvalue_6 _returnvalue_6))
    (bind _returnvalue_7 (/ _returnvalue_3 2.0))
    (bind _returnvalue_8 (+ (+ (`self.Padding`) _returnvalue_7) (`self.LastAddedComponentDistRight`)))
    (`self.K2_SetActorLocationAndRotation` :`self` _widget_2 :`NewLocation` (`KismetMathLibrary.MakeVector` (/ (+ (.x _returnvalue) (.x (`SceneComponent.K2_GetComponentLocation` (`self.DefaultSceneRoot`)))) 2.0) (- (.y _returnvalue) (* _returnvalue_6 _returnvalue_8)) (+ (.z _returnvalue) (+ (/ _returnvalue_5 2.0) (`self.Padding`)))))
    (bind _asmovable_widget_bp_2 (cast `/Game/Blueprints/Widget_BP/MovableWidget_BP` _widget_2))
    (bind _returnvalue_9 (`SceneComponent.K2_GetComponentLocation` (`/Game/Blueprints/Widget_BP/MovableWidget_BP.LeftDownPos_Wid` _asmovable_widget_bp_2)))
    (bind _returnvalue_10 (`SceneComponent.K2_GetComponentLocation` (`/Game/Blueprints/Widget_BP/MovableWidget_BP.RightDownPos_Wid` _asmovable_widget_bp_2)))
    (bind _returnvalue_11 (`SceneComponent.K2_GetComponentLocation` (`/Game/Blueprints/Widget_BP/MovableWidget_BP.RightUpPos_Wid` _asmovable_widget_bp_2)))
    (`KismetArrayLibrary.Array_Add` (`self.NewArrayOfWidgets`) (make `/Game/Blueprints/Widget_BP/ArrayOfWidgetsOnTheDisplay` _widget_2 _returnvalue_9 _returnvalue_10 (`SceneComponent.K2_GetComponentLocation` (`/Game/Blueprints/Widget_BP/MovableWidget_BP.LeftUpPos_Wid` _asmovable_widget_bp_2)) _returnvalue_11 (`KismetMathLibrary.Vector_Distance` _returnvalue_10 _returnvalue_11) (`KismetMathLibrary.Vector_Distance` _returnvalue_9 _returnvalue_10) _previousscale))
    (set `self.LastAddedComponentDistRight` (+ _returnvalue_8 _returnvalue_7)))
  (set `self.ArrayOfLeft` 0.0)
  (set `self.ArrayOfUp` 0.0)
  (return (`self.NewArrayOfWidgets`)))

(fn `UserConstructionScript`)