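; Vive motion controller rig for a coupled-tanks mixed-reality scene, enabling ViveSR's depth collider mesh on BeginPlay.
; Right trigger line traces level planes, converting hits into tank height values for MATLAB.
; Right grip traces and attaches models, which face buttons rotate and raise, levelling them on release.
; Left grip grabs interface actors, letting right grip resize them, while hand skeletons replace controller meshes near pickup spheres.
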(event `self.ReceiveBeginPlay`
  (bind _dualcameradepthcollider (`ViveSR.DualCameraDepthCollider` (`self.ViveSR`)))
  (bind _mesh (`ViveSR_DualCameraDepthCollider.mesh` (`ViveSR.DualCameraDepthCollider` (`self.ViveSR`))))
  ;[1 1 1] BeginPlay
  (`|ExecutionSequence`
    (:`then_0`
      ;[1 1 1] Get ViveSR Reference
      (bind _returnvalue (`GameplayStatics.LoadGameFromSlot` "ViveSRSlot"))
      (bind _asexperience_save_game (cast `/Game/CoupledTanksProject/Blueprints/Experience_SaveGame` _returnvalue))
      (set `self.ViveSR` (`/Game/CoupledTanksProject/Blueprints/Experience_SaveGame.ViveSR` _asexperience_save_game)))
    (:`then_3`
      ;[1 1 1] Turn On Dynamic Mesh
      (`SRWorksFunctionLibrary.EnableDepthProcess` true)
      (`ViveSR_DualCameraDepthCollider.SetColliderProcessEnable` _dualcameradepthcollider true)
      (`ViveSR_DualCameraDepthCollider.SetLiveMeshVisibility` _dualcameradepthcollider (`self.ShowDynamicMesh`))
      (`PrimitiveComponent.SetMaterial` _mesh 0 (`.MaterialInterface` (break `StaticMaterial` (`self.WireframeMat`))))
      (`PrimitiveComponent.SetCollisionEnabled` _mesh "QueryAndPhysics"))))

(event `self.ReceiveTick`
  (params (DeltaSeconds :type "Float (single-precision)"))
  (bind _right (`self.Right`))
  (bind _right_2 (`self.Right`))
  (bind _returnvalue (`SceneComponent.K2_GetComponentLocation` _right))
  (bind _returnvalue_2 (`SceneComponent.K2_GetComponentLocation` _right_2))
  (bind _returnvalue_3 (`MotionControllerComponent.IsTracked` (`self.Right`)))
  (bind _returnvalue_4 (`MotionControllerComponent.IsTracked` (`self.Left`)))
  ;[1 1 1] Tick
  (`|ExecutionSequence`
    (:`then_0`
      ;[1 1 1] Set Camera Shift
      (`SceneComponent.K2_SetRelativeLocation` (`self.Scene`) (* (`SceneComponent.GetForwardVector` (`self.VRCamera`)) 7.1) false false))
    (:`then_1`
      ;[1 1 1] Set Controller Visibility
      (`|ExecutionSequence`
        (:`then_0`
          (if (!= _returnvalue_4 (`self.OldVisibilityL`))
            (`SceneComponent.SetVisibility` (`self.L_Mesh`) _returnvalue_4 true)
            (set `self.OldVisibilityL` _returnvalue_4)))
        (:`then_1`
          (if (!= _returnvalue_3 (`self.OldVisibilityR`))
            (`SceneComponent.SetVisibility` (`self.R_Mesh`) _returnvalue_3 true)
            (set `self.OldVisibilityR` _returnvalue_3)))))
    (:`then_2`
      ;[1 1 1] Reflect Player Thumb Location on Touchpad
      (`SceneComponent.K2_SetRelativeLocation` (`self.finger`) (`KismetMathLibrary.MakeVector` (`KismetMathLibrary.MapRangeUnclamped` (`self.GetInputAxisKeyValue`) -1.0 1.0 1.8 -1.8) (`KismetMathLibrary.MapRangeUnclamped` (`self.GetInputAxisKeyValue`) -1.0 1.0 -1.8 1.8)) false false))
    (:`then_3`
      ;[1 1 1] LineTrace from controller
      (if (`self.ActorIsGrabbed`)
        _
        (elif (`self.R Trigger Pressed`)
          (bind (_outhit _returnvalue_5) (`KismetSystemLibrary.LineTraceSingleForObjects` :`Start` _returnvalue :`End` (+ _returnvalue (* (`KismetMathLibrary.GetForwardVector` (`SceneComponent.K2_GetComponentRotation` _right)) (`self.MainLineTraceLength`))) :`ObjectTypes` (`|MakeArray` "ObjectTypeQuery7" :!type "EObjectTypeQuery Enum") :`DrawDebugType` "ForOneFrame" :`TraceColor` (struct :`G` 0.8 :`B` 1.0 :`A` 1.0) :`DrawTime` 1.0))
          (if _returnvalue_5
            (bind (_bblockinghit _binitialoverlap _time _distance _location _impactpoint _normal _impactnormal _physmat _hitactor) (`GameplayStatics.BreakHitResult` _outhit))
            (bind _asbp_level_controller_plane (cast `/Game/CoupledTanksProject/Blueprints/BP_Level_Controller_Plane` _hitactor))
            ;[1 1 1] Check the ID of the tank and set the corresponding value for further transmit
            (switch `int` (`/Game/CoupledTanksProject/Blueprints/BP_Level_Controller_Plane.TankID` _asbp_level_controller_plane)
              (:`1`
                (bind _returnvalue_6 (* 0.25 (/ (- (`KismetMathLibrary.Abs` (.x (`KismetMathLibrary.InverseTransformLocation` (`self.GetTransform` _asbp_level_controller_plane) _location))) 0.0) (- (.x (`.Max` (`StaticMeshComponent.GetLocalBounds` (`/Game/CoupledTanksProject/Blueprints/BP_Level_Controller_Plane.coll_plane` _asbp_level_controller_plane)))) 0.0))))
                (set `self.tank1H` _returnvalue_6))
              (:`2`
                (set `self.tank2H` _returnvalue_6))
              (:`3`
                (set `self.tank3H` _returnvalue_6)))
            (bind _returnvalue_7 (`KismetMathLibrary.VSize` (- _location (`SceneComponent.K2_GetComponentLocation` (`self.Right`)))))
            ;[1 1 1] If Linetrace hits an object of required type it no longer "cuts through" it
            (if (< _returnvalue_7 200.0)
              (set `self.MainLineTraceLength` (+ _returnvalue_7 1.5)))
            (else
              (set `self.MainLineTraceLength` 200.0))))))
    (:`then_4`
      ;[1 1 1] LineTrace from controller
      (if (`self.ActorIsGrabbed`)
        _
        (elif (`self.R Grip Pressed`)
          (bind (_outhit_2 _returnvalue_8) (`KismetSystemLibrary.LineTraceSingleForObjects` :`Start` _returnvalue_2 :`End` (+ _returnvalue_2 (* (`KismetMathLibrary.GetForwardVector` (`SceneComponent.K2_GetComponentRotation` _right_2)) (`self.SecondaryLineTraceLength`))) :`ObjectTypes` (`|MakeArray` "ObjectTypeQuery8" :!type "EObjectTypeQuery Enum") :`DrawDebugType` "ForOneFrame" :`TraceColor` (struct :`R` 1.0 :`G` 0.789114 :`A` 1.0) :`DrawTime` 1.0))
          (if _returnvalue_8
            (bind (_bblockinghit_2 _binitialoverlap_2 _time_2 _distance_2 _location_2 _impactpoint_2 _normal_2 _impactnormal_2 _physmat_2 _hitactor_2) (`GameplayStatics.BreakHitResult` _outhit_2))
            ;[1 1 1] Attach object to right controller to move it freely along X and Y
            (`self.K2_AttachToComponent` _hitactor_2 (`self.R_Mesh`) "None" "KeepWorld" "KeepWorld" "KeepWorld" true)
            (bind _output_get (set `self.AttachedActorRef` _hitactor_2))
            (set `self.ActorAttached` true)
            (bind _returnvalue_9 (`KismetMathLibrary.VSize` (- _location_2 (`SceneComponent.K2_GetComponentLocation` (`self.Right`)))))
            ;[1 1 1] If Linetrace hits an object of required type it no longer "cuts through" it
            (if (< _returnvalue_9 200.0)
              (set `self.SecondaryLineTraceLength` (+ _returnvalue_9 1.5)))
            (elif (not (`self.ActorAttached`))
              (set `self.SecondaryLineTraceLength` 200.0))))))
    (:`then_5`
      ;[1 1 1] Check whether attached object is NULL
      (if (!= (`self.AttachedActorRef`) null)
        ;[1 1 1] Rotate every frame by 1deg while controller FaceButton 2 or 4  is pressed
        (`|ExecutionSequence`
          (:`then_0`
            (if (`self.R FaceButton2 Pressed`)
              (bind _returnvalue_10 (`self.K2_GetActorRotation` _output_get))
              (`self.K2_SetActorRotation` _output_get (`KismetMathLibrary.MakeRotator` (.roll _returnvalue_10) (.pitch _returnvalue_10) (+ (.yaw _returnvalue_10) 1.0)) false)))
          (:`then_1`
            (if (`self.R FaceButton4 Pressed`)
              (`self.K2_SetActorRotation` _output_get (`KismetMathLibrary.MakeRotator` (.roll _returnvalue_10) (.pitch _returnvalue_10) (- (.yaw _returnvalue_10) 1.0)) false)))
          (:`then_2`
            ;[1 1 1] Move up/down every frame by 1 while controller FaceButton 1 or 3 is pressed
            (if (`self.R FaceButton1 Pressed`)
              (bind _returnvalue_11 (`self.K2_GetActorLocation` _output_get))
              (bind _returnvalue_12 (+ (.z _returnvalue_11) 1.0))
              (set `self.Custom Z Value of Model` _returnvalue_12)
              (`self.K2_SetActorLocation` _output_get (`KismetMathLibrary.MakeVector` (.x _returnvalue_11) (.y _returnvalue_11) _returnvalue_12) false false)))
          (:`then_3`
            (if (`self.R FaceButton3 Pressed`)
              (bind _returnvalue_13 (- (.z _returnvalue_11) 1.0))
              (set `self.Custom Z Value of Model` _returnvalue_13)
              (`self.K2_SetActorLocation` _output_get (`KismetMathLibrary.MakeVector` (.x _returnvalue_11) (.y _returnvalue_11) _returnvalue_13) false false))))))
    (:`then_6`
      (if (not (!= (`self.AttachedActor`) null))
        (`self.GetActorNearHand`)))
    (:`then_7`
      (`self.HandleHandOverlapSphere`))))

(event `Key|MotionController_Left_Grip1`
  (params (Key :type "Key Structure"))
  (:`Pressed`
    (`self.GrabActor`))
  (:`Released`
    (`self.ReleaseActor`)))

(event `HandleHandOverlapSphere`
  (if (> (`KismetArrayLibrary.Array_Length` (`PrimitiveComponent.GetOverlappingActors` (`self.GrabSph`) "/Game/CoupledTanksProject/Blueprints/BP_PickupAndResizeSphere.BP_PickupAndResizeSphere_C")) 0)
    (`SceneComponent.SetVisibility` (`self.LefhHandSkeleton`) true false)
    (`SceneComponent.SetVisibility` (`self.RightHandSkeleton`) true false)
    (`SceneComponent.SetVisibility` (`self.L_Mesh`) false false)
    (`SceneComponent.SetVisibility` (`self.R_Mesh`) false false)
    (else
      (`SceneComponent.SetVisibility` (`self.LefhHandSkeleton`) false false)
      (`SceneComponent.SetVisibility` (`self.RightHandSkeleton`) false false)
      (`SceneComponent.SetVisibility` (`self.L_Mesh`) true false)
      (`SceneComponent.SetVisibility` (`self.R_Mesh`) true false))))

(event `Key|MotionController_Right_Trigger`
  (params (Key :type "Key Structure"))
  ;[1 1 1] Change "R Trigger Pressed" value
  (:`Pressed`
    (set `self.R Trigger Pressed` true))
  (:`Released`
    (set `self.R Trigger Pressed` false)))

(event `Key|MotionController_Right_Grip1`
  (params (Key :type "Key Structure"))
  (bind _attachedactorref (`self.AttachedActorRef`))
  (bind _attachedactorref_2 (`self.AttachedActorRef`))
  ;[1 1 1] Change "R Grip Pressed" value
  (:`Pressed`
    (set `self.R Grip Pressed` true)
    (if (`self.ActorIsGrabbed`)
      (`self.StartResizeActor` (`self.Right`))
      (bind _asright_hand_anim_bpcustom (cast `/Game/VirtualReality/Mannequin/Animations/RightHand_AnimBPCustom` (`SkeletalMeshComponent.GetAnimInstance` (`self.RightHandSkeleton`))))
      (set `/Game/VirtualReality/Mannequin/Animations/RightHand_AnimBPCustom.GripState` "NewEnumerator2" _asright_hand_anim_bpcustom)))
  (:`Released`
    (set `self.R Grip Pressed` false)
    (`self.EndResizeActor`)
    (bind _asright_hand_anim_bpcustom_2 (cast `/Game/VirtualReality/Mannequin/Animations/RightHand_AnimBPCustom` (`SkeletalMeshComponent.GetAnimInstance` (`self.RightHandSkeleton`))))
    (set `/Game/VirtualReality/Mannequin/Animations/RightHand_AnimBPCustom.GripState` "NewEnumerator0" _asright_hand_anim_bpcustom_2)
    (if (!= _attachedactorref_2 null)
      (`SceneComponent.K2_DetachFromComponent` (`Actor.RootComponent` _attachedactorref) "KeepWorld" "KeepWorld" "KeepWorld" true)
      (`self.K2_SetActorTransform` _attachedactorref (`KismetMathLibrary.MakeTransform` (`KismetMathLibrary.MakeVector` (.x (.location (`self.GetTransform` _attachedactorref_2))) (.y (.location (`self.GetTransform` _attachedactorref_2))) (`self.Custom Z Value of Model`)) (`KismetMathLibrary.MakeRotator` 0.0 0.0 (.yaw (.rotation (`self.GetTransform` _attachedactorref_2)))) (.scale (`self.GetTransform` _attachedactorref_2))) false false)
      (set `self.AttachedActorRef` (`self.NullActorRef`))
      (set `self.ActorAttached` false))))

(event `Key|MotionController_Right_FaceButton2`
  (params (Key :type "Key Structure"))
  ;[1 1 1] Change "R nFaceButton Pressed" value
  (:`Pressed`
    (set `self.R FaceButton2 Pressed` true))
  (:`Released`
    (set `self.R FaceButton2 Pressed` false)))

(event `Key|MotionController_Right_FaceButton4`
  (params (Key :type "Key Structure"))
  ;[1 1 1] Change "R nFaceButton Pressed" value
  (:`Pressed`
    (set `self.R FaceButton4 Pressed` true))
  (:`Released`
    (set `self.R FaceButton4 Pressed` false)))

(event `Key|MotionController_Right_FaceButton1`
  (params (Key :type "Key Structure"))
  ;[1 1 1] Change "R nFaceButton Pressed" value
  (:`Pressed`
    (set `self.R FaceButton1 Pressed` true))
  (:`Released`
    (set `self.R FaceButton1 Pressed` false)))

(event `Key|MotionController_Right_FaceButton3`
  (params (Key :type "Key Structure"))
  ;[1 1 1] Change "R nFaceButton Pressed" value
  (:`Pressed`
    (set `self.R FaceButton3 Pressed` true))
  (:`Released`
    (set `self.R FaceButton3 Pressed` false)))

(fn `EndResizeActor`
  (message `/Game/CoupledTanksProject/Blueprints/BP_PickupAndResizeActorInterface.EndResize` (`self.ResizedActor`)))

(fn `GetActorNearHand`
  (returns (NearestMesh :type "Actor Object Reference"))
  (locals (NearestOverlappingActor :type "Actor Object Reference") (NearestOverlap :type "Float (double-precision)"))
  (bind _grabsph (`self.GrabSph`))
  (for _array_element (`PrimitiveComponent.GetOverlappingActors` _grabsph "/Script/Engine.Actor")
    (if (`KismetSystemLibrary.DoesImplementInterface` _array_element "/Game/CoupledTanksProject/Blueprints/BP_PickupAndResizeActorInterface.BP_PickupAndResizeActorInterface_C")
      (set `local.NearestOverlappingActor` _array_element)
      (set `local.NearestOverlap` (`KismetMathLibrary.VSize` (- (`self.K2_GetActorLocation` _array_element) (`SceneComponent.K2_GetComponentLocation` _grabsph))))))
  (return (`local.NearestOverlappingActor`)))

(fn `GrabActor`
  (bind _nearestmesh (`self.GetActorNearHand`))
  (`/Engine/EditorBlueprintResources/StandardMacros.IsValid` _nearestmesh
    (:`Is Valid`
      (set `self.AttachedActor` _nearestmesh)
      (bind _asright_hand_anim_bpcustom (cast `/Game/VirtualReality/Mannequin/Animations/RightHand_AnimBPCustom` (`SkeletalMeshComponent.GetAnimInstance` (`self.LefhHandSkeleton`))))
      (set `/Game/VirtualReality/Mannequin/Animations/RightHand_AnimBPCustom.GripState` "NewEnumerator2" _asright_hand_anim_bpcustom)
      (message `/Game/CoupledTanksProject/Blueprints/BP_PickupAndResizeActorInterface.Pickup` _nearestmesh (`self.Left`))
      (set `self.ActorIsGrabbed` true))))

(fn `ReleaseActor`
  (bind _attachedactor (`self.AttachedActor`))
  (`/Engine/EditorBlueprintResources/StandardMacros.IsValid` _attachedactor
    (:`Is Valid`
      (if (== (`SceneComponent.GetAttachParent` (`self.K2_GetRootComponent` _attachedactor)) (`self.Left`))
        (message `/Game/CoupledTanksProject/Blueprints/BP_PickupAndResizeActorInterface.Drop` _attachedactor))
      (set `self.AttachedActor` null) ; Clear the reference
      (set `self.ActorIsGrabbed` false)
      (bind _asright_hand_anim_bpcustom (cast `/Game/VirtualReality/Mannequin/Animations/RightHand_AnimBPCustom` (`SkeletalMeshComponent.GetAnimInstance` (`self.LefhHandSkeleton`))))
      (set `/Game/VirtualReality/Mannequin/Animations/RightHand_AnimBPCustom.GripState` "NewEnumerator0" _asright_hand_anim_bpcustom))))

(fn `StartResizeActor`
  (params (OtherHand :type "MotionControllerComponent Object Reference"))
  (bind _nearestmesh (`self.GetActorNearHand`))
  (`/Engine/EditorBlueprintResources/StandardMacros.IsValid` _nearestmesh
    (:`Is Valid`
      (bind _output_get (set `self.ResizedActor` (`self.AttachedActor`)))
      (message `/Game/CoupledTanksProject/Blueprints/BP_PickupAndResizeActorInterface.StartResize` _output_get (`self.Left`) OtherHand))))

(fn `SwitchLevel`
  (locals (targetLevelNum :type Integer))
  (bind _returnvalue (+ (`self.LevelNum`) 1))
  (`|ExecutionSequence`
    (:`then_0`
      ;[1 1 1] Switch off current level
      (set `LevelStreaming.bShouldBeVisible` false (`GameplayStatics.GetStreamingLevel` (`|GetArrayItem` (`self.LevelName`) (`self.LevelNum`)))))
    (:`then_1`
      ;[1 1 1] Switch on next level
      (set `local.targetLevelNum` (`KismetMathLibrary.SelectInt` 0 _returnvalue (== _returnvalue (`KismetArrayLibrary.Array_Length` (`self.LevelName`)))))
      (set `LevelStreaming.bShouldBeVisible` true (`GameplayStatics.GetStreamingLevel` (`|GetArrayItem` (`self.LevelName`) (`local.targetLevelNum`)))))))

(fn `UserConstructionScript`)