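; VR sphere in the coupled-tanks project that motion controllers pick up and resize to set a P or I parameter, chosen by ParameterID.
; Two-hand resizing scales the inner sphere by the change in hand distance, clamped between limits, with haptics at either limit.
; InterpolateValue linearly maps that scale to the parameter range and passes it to TanksUdpSend.
; The actor yaws toward the VR camera and swaps material on controller overlap.
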(event `self.ReceiveBeginPlay`
  (bind _symbol (`self.Symbol`))
  (bind _outersphereinitialscale_innerspheremaxscale_value (`self.OuterSphereInitialScale(InnerSphereMaxScale)Value`))
  (bind _mininnerspherescalevalue (`self.MinInnerSphereScaleValue`))
  (bind _maxinnerspherescalevalue (`self.MaxInnerSphereScaleValue`))
  (switch `int` (`self.ParameterID`)
    (:`Default`
      (`StaticMeshComponent.SetStaticMesh` _symbol "/Game/CoupledTanksProject/Meshes/Symbol_P.Symbol_P" :!label _label))
    (:`0`
      (goto _label))
    (:`1`
      (`StaticMeshComponent.SetStaticMesh` _symbol "/Game/CoupledTanksProject/Meshes/Symbol_I.Symbol_I")))
  ;[1 1 1] Outer Sphere Scale >= (positive non-zero value)
  (set `self.OuterSphereInitialScale` (`KismetMathLibrary.Conv_DoubleToVector` _outersphereinitialscale_innerspheremaxscale_value))
  ;[1 1 1] Inner sphere max scale is in bounds of outer sphere scale
  (set `self.MaxInnerSphereScaleValue` _outersphereinitialscale_innerspheremaxscale_value)
  (if (>= _mininnerspherescalevalue _maxinnerspherescalevalue)
    ;[1 1 1] Set MinInnerSphereScale to 90% of MaxInnerSphereScale if Min Inner Sphere Scale is bigged that or equal to Max Inner Sphere Scale
    (set `self.MinInnerSphereScaleValue` (* (`self.MaxInnerSphereScaleValue`) 0.9)))
  ;[1 1 1] Clamp InnerSphereInitialScale between min and max scales
  (set `self.InnerSphereInitialScale` (`KismetMathLibrary.Conv_DoubleToVector` (`KismetMathLibrary.FClamp` (`self.InnerSphereInitialScaleValue`) _mininnerspherescalevalue _maxinnerspherescalevalue)))
  (`PrimitiveComponent.SetMaterial` (`self.StaticMeshComponent`) 0 (`self.DefaultMaterial`))
  ;[1 1 1] Set the initial scale of spheres
  (`SceneComponent.SetWorldScale3D` (`self.StaticMeshComponent`) (`self.OuterSphereInitialScale`))
  (`SceneComponent.SetWorldScale3D` (`self.InnerSphere`) (`self.InnerSphereInitialScale`))
  (`self.InterpolateValue`))

(event `/Game/CoupledTanksProject/Blueprints/BP_PickupAndResizeActorInterface.StartResize`
  (params (FirstHand :type "MotionControllerComponent Object Reference") (SecondHand :type "MotionControllerComponent Object Reference"))
  (set `self.FirstHand` FirstHand)
  (set `self.SecondHand` SecondHand)
  (set `self.SphereResizing` true)
  (set `self.InitialDistance` (`KismetMathLibrary.Abs` (`KismetMathLibrary.VSize` (- (`SceneComponent.K2_GetComponentLocation` (`self.FirstHand`)) (`SceneComponent.K2_GetComponentLocation` (`self.SecondHand`))))))
  (set `self.InitialScale` (`SceneComponent.K2_GetComponentScale` (`self.InnerSphere`))))

(event `self.ReceiveTick`
  (params (DeltaSeconds :type "Float (single-precision)"))
  (bind _mininnerspherescalevalue (`self.MinInnerSphereScaleValue`))
  (bind _maxinnerspherescalevalue (`self.MaxInnerSphereScaleValue`))
  (bind _maxinnerspherescalevalue_2 (`self.MaxInnerSphereScaleValue`))
  (bind _mininnerspherescalevalue_2 (`self.MinInnerSphereScaleValue`))
  (bind _returnvalue (`KismetMathLibrary.MakeVector` (`KismetMathLibrary.FClamp` (.x (* (`self.InitialScale`) (/ (`KismetMathLibrary.Abs` (`KismetMathLibrary.VSize` (- (`SceneComponent.K2_GetComponentLocation` (`self.FirstHand`)) (`SceneComponent.K2_GetComponentLocation` (`self.SecondHand`))))) (`self.InitialDistance`)))) _mininnerspherescalevalue _maxinnerspherescalevalue) (`KismetMathLibrary.FClamp` (.y (* (`self.InitialScale`) (/ (`KismetMathLibrary.Abs` (`KismetMathLibrary.VSize` (- (`SceneComponent.K2_GetComponentLocation` (`self.FirstHand`)) (`SceneComponent.K2_GetComponentLocation` (`self.SecondHand`))))) (`self.InitialDistance`)))) _mininnerspherescalevalue _maxinnerspherescalevalue) (`KismetMathLibrary.FClamp` (.z (* (`self.InitialScale`) (/ (`KismetMathLibrary.Abs` (`KismetMathLibrary.VSize` (- (`SceneComponent.K2_GetComponentLocation` (`self.FirstHand`)) (`SceneComponent.K2_GetComponentLocation` (`self.SecondHand`))))) (`self.InitialDistance`)))) _mininnerspherescalevalue _maxinnerspherescalevalue)))
  (`self.K2_SetActorRotation` (`KismetMathLibrary.MakeRotator` 0.0 0.0 (.yaw (`KismetMathLibrary.FindLookAtRotation` (`self.K2_GetActorLocation`) (`SceneComponent.K2_GetComponentLocation` (`/Game/CoupledTanksProject/Blueprints/BP_Tanks_CustomViveMotionController.VRCamera` (`self.BP_Tanks_CustomViveMotionControllerRef`)))))))
  (if (`self.SphereResizing`)
    (bind _output_get (set `self.InnerSphereInitialScale` _returnvalue))
    (`SceneComponent.SetWorldScale3D` (`self.InnerSphere`) _output_get)
    (`self.InterpolateValue`)
    (if (or (`KismetMathLibrary.EqualExactly_VectorVector` _returnvalue (`KismetMathLibrary.MakeVector` _mininnerspherescalevalue_2 _mininnerspherescalevalue_2 _mininnerspherescalevalue_2)) (`KismetMathLibrary.EqualExactly_VectorVector` _returnvalue (`KismetMathLibrary.MakeVector` _maxinnerspherescalevalue_2 _maxinnerspherescalevalue_2 _maxinnerspherescalevalue_2)))
      (`PlayerController.PlayHapticEffect` (`GameplayStatics.GetPlayerController` 0) "/Game/CoupledTanksProject/Blueprints/MigratedContent/MotionControllerHapticsCustom.MotionControllerHapticsCustom" "Left" 1.0 false)
      (`PlayerController.PlayHapticEffect` (`GameplayStatics.GetPlayerController` 0) "/Game/CoupledTanksProject/Blueprints/MigratedContent/MotionControllerHapticsCustom.MotionControllerHapticsCustom" "Right" 1.0 false))))

(event `/Game/CoupledTanksProject/Blueprints/BP_PickupAndResizeActorInterface.EndResize`
  (set `self.SphereResizing` false))

(event `/Game/CoupledTanksProject/Blueprints/BP_PickupAndResizeActorInterface.Pickup`
  (params (`Attach To ` :type "SceneComponent Object Reference"))
  (`self.K2_DetachFromActor` "KeepWorld" "KeepWorld" "KeepWorld")
  (`SceneComponent.K2_AttachToComponent` (`self.K2_GetRootComponent`) `Attach To ` "None" "KeepWorld" "KeepWorld" "KeepWorld" false))

(event `/Game/CoupledTanksProject/Blueprints/BP_PickupAndResizeActorInterface.Drop`
  (`self.K2_DetachFromActor` "KeepWorld" "KeepWorld" "KeepWorld"))

(event `self.ReceiveActorBeginOverlap`
  (params (OtherActor :type "Actor Object Reference"))
  (cast `/Game/CoupledTanksProject/Blueprints/BP_Tanks_CustomViveMotionController` OtherActor)
  (`PrimitiveComponent.SetMaterial` (`self.StaticMeshComponent`) 0 (`self.InteractableMaterial`)))

(event `self.ReceiveActorEndOverlap`
  (params (OtherActor :type "Actor Object Reference"))
  (cast `/Game/CoupledTanksProject/Blueprints/BP_Tanks_CustomViveMotionController` OtherActor)
  (`PrimitiveComponent.SetMaterial` (`self.StaticMeshComponent`) 0 (`self.DefaultMaterial`)))

(event `InterpolateValue`
  (bind _tanksudpsend (`self.TanksUdpSend`))
  ;[1 1 1] Interpolation formula: x = (D-C)[(y - A)/(B - A)] + C
  (switch `int` (`self.ParameterID`)
    (:`Default`
      (bind _interpolatedp (`self.Linear Interpolation For Parameter P` :!label _label_2))
      (set `/Game/CoupledTanksProject/Blueprints/BP_TanksUdpSend.SphereScaleToBeSent_Sphere1` _interpolatedp _tanksudpsend))
    (:`0`
      (goto _label_2))
    (:`1`
      (bind _interpolatedi (`self.Linear Interpolation For Parameter I`))
      (set `/Game/CoupledTanksProject/Blueprints/BP_TanksUdpSend.SphereScaleToBeSent_Sphere2` _interpolatedi _tanksudpsend))))

(fn `Linear Interpolation For Parameter I`
  (returns (InterpolatedI :type "Float (double-precision)"))
  (return (`KismetMathLibrary.Abs` (+ (* (- (`self.D (I param Interpolation)`) (`self.C (I param Interpolation)`)) (/ (- (.x (`self.InnerSphereInitialScale`)) (`self.MinInnerSphereScaleValue`)) (- (`self.MaxInnerSphereScaleValue`) (`self.MinInnerSphereScaleValue`)))) (`self.C (I param Interpolation)`)))))

(fn `Linear Interpolation For Parameter P`
  (returns (InterpolatedP :type "Float (double-precision)"))
  (return (`KismetMathLibrary.Abs` (+ (* (- (`self.D (P param Interpolation)`) (`self.C (P param Interpolation)`)) (/ (- (.x (`self.InnerSphereInitialScale`)) (`self.MinInnerSphereScaleValue`)) (- (`self.MaxInnerSphereScaleValue`) (`self.MinInnerSphereScaleValue`)))) (`self.C (P param Interpolation)`)))))

(fn `UserConstructionScript`)