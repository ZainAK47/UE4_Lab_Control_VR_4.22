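; Receives UDP data for a three-tank coupled-tanks simulation and visualizes each tank's liquid level.
; Starts a receiver on BeginPlay, then on Tick reads each tank's lowest-point socket and checks for new data.
; Three floats set the height of BP_Hider1–3 planes as socket Z plus the scaled level, and a fourth is stored as the received integral parameter.
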(event `self.ReceiveBeginPlay`
  (bind _returnvalue (`self.StartUDPReceiver` "sock1" 9988))
  (set `self.UDPReceiver started` _returnvalue))

(event `self.ReceiveTick`
  (params (DeltaSeconds :type "Float (single-precision)"))
  (`|ExecutionSequence`
    (:`then_0`
      (set `self.Tank1LowestPoint` (.z (`SceneComponent.GetSocketLocation` (`/Game/CoupledTanksProject/Blueprints/BP_Tank_Parent_Liquid.Tank_Shape` (`self.Tank1_Liquid`)) "Lowest Point Tank1"))))
    (:`then_1`
      (set `self.Tank2LowestPoint` (.z (`SceneComponent.GetSocketLocation` (`/Game/CoupledTanksProject/Blueprints/BP_Tank_Parent_Liquid.Tank_Shape` (`self.Tank2_Liquid`)) "Lowest Point Tank2"))))
    (:`then_2`
      (set `self.Tank3LowestPoint` (.z (`SceneComponent.GetSocketLocation` (`/Game/CoupledTanksProject/Blueprints/BP_Tank_Parent_Liquid.Tank_Shape` (`self.Tank3_Liquid`)) "Lowest Point Tank3")))))
  (bind _returnvalue (`self.IsNewDataReady`))
  (if _returnvalue
    (bind _returnvalue_2 (`self.GetData`))
    (`|ExecutionSequence`
      (:`then_0`
        (bind (_float1 _float2 _float3 _float4) (break `UDPData` _returnvalue_2))
        (`self.Tank 1 Level Change` _float1 _float1))
      (:`then_1`
        (`self.Tank 2 Level Change` _float2 _float2))
      (:`then_2`
        (`self.Tank 3 Level Change` _float3 _float3))
      (:`then_3`
        (set `self.ReceivedIntegralParameter` _float4)))))

(fn `UserConstructionScript`)