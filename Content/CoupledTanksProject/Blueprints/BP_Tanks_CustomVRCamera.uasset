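; Custom VR camera Blueprint for the Coupled Tanks project, handling a camera offset and a touchpad finger indicator.
; On BeginPlay it caches the ViveSR value from the Experience save game slot.
; Each tick it offsets HMDCameraShifter along the VR camera's forward and up vectors by configurable shift amounts.
; It also remaps input axes to move the Finger component, mirroring the player's thumb position on the touchpad.
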(event `self.ReceiveBeginPlay`
  (`|ExecutionSequence`
    (:`then_0`
      ;[1 1 1] Get ViveSR Reference
      (bind _returnvalue (`GameplayStatics.LoadGameFromSlot` "ViveSRSlot"))
      (bind _asexperience_save_game (cast `/Game/CoupledTanksProject/Blueprints/Experience_SaveGame` _returnvalue))
      (set `self.ViveSR` (`/Game/CoupledTanksProject/Blueprints/Experience_SaveGame.ViveSR` _asexperience_save_game)))))

(event `self.ReceiveTick`
  (params (DeltaSeconds :type "Float (single-precision)"))
  (`|ExecutionSequence`
    (:`then_0`
      (`SceneComponent.K2_SetRelativeLocation` (`self.HMDCameraShifter`) (+ (* (`SceneComponent.GetForwardVector` (`self.VRCamera`)) (`self.CameraShiftZ`)) (* (`SceneComponent.GetUpVector` (`self.VRCamera`)) (`self.CameraShiftY`))) false false))
    (:`then_1`
      ;[1 1 1] Reflect Player Thumb Location on Touchpad
      (`SceneComponent.K2_SetRelativeLocation` (`self.Finger`) (`KismetMathLibrary.MakeVector` (`KismetMathLibrary.MapRangeUnclamped` (`self.GetInputAxisKeyValue`) -1.0 1.0 1.8 -1.8) (`KismetMathLibrary.MapRangeUnclamped` (`self.GetInputAxisKeyValue`) -1.0 1.0 -1.8 1.8)) false false))))

(fn `UserConstructionScript`)