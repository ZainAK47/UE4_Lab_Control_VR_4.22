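; Actor Blueprint that feeds live coupled-tank data into chart widgets in the world.
; Every Tick it searches for all TanksMovableWidget_BP actors and checks each one's widget class.
; TanksRealGraph_Widget gets tank setpoints from CustomViveMotionController and measured levels from TanksUDPRecv, though the Tank 3 setpoint node is unconnected.
; BarChart_Widget gets the received integral parameter from TanksUDPRecv.
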(event `self.ReceiveTick`
  (params (DeltaSeconds :type "Float (single-precision)"))
  (bind _outactors (`GameplayStatics.GetAllActorsOfClass` "/Game/CoupledTanksProject/Blueprints/TanksMovableWidget_BP.TanksMovableWidget_BP_C"))
  (for (_ _array_index) _outactors
    (`|ExecutionSequence`
      (:`then_0`
        (bind _output (`|GetArrayItem` _outactors _array_index))
        (bind _returnvalue (`WidgetComponent.GetUserWidgetObject` (`/Game/CoupledTanksProject/Blueprints/TanksMovableWidget_BP.Widget` _output)))
        (if (== (`GameplayStatics.GetObjectClass` _returnvalue) "/Game/CoupledTanksProject/Blueprints/TanksRealGraph_Widget.TanksRealGraph_Widget_C")
          (bind _astanks_real_graph_widget (cast `/Game/CoupledTanksProject/Blueprints/TanksRealGraph_Widget` _returnvalue))
          (`|ExecutionSequence`
            (:`then_0`
              ;[1 1 1] Tank 1 Liquid Level Manually Set Point
              (`/Game/CoupledTanksProject/Blueprints/TanksRealGraph_Widget.AddDesiredHeightTank1` _astanks_real_graph_widget (`/Game/CoupledTanksProject/Blueprints/BP_Tanks_CustomViveMotionController.tank1H` (`self.CustomViveMotionController`)))
              ;[1 1 1] Tank 1 Liquid Level In Real Object
              (`/Game/CoupledTanksProject/Blueprints/TanksRealGraph_Widget.AddActualHeightTank1` _astanks_real_graph_widget (`/Game/CoupledTanksProject/Blueprints/BP_TanksUdpRecv.Tank1ReceivedValue` (`self.TanksUDPRecv`))))
            (:`then_1`
              ;[1 1 1] Tank 2 Liquid Level Manually Set Point
              (`/Game/CoupledTanksProject/Blueprints/TanksRealGraph_Widget.AddDesiredHeightTank2` _astanks_real_graph_widget (`/Game/CoupledTanksProject/Blueprints/BP_Tanks_CustomViveMotionController.tank2H` (`self.CustomViveMotionController`)))
              ;[1 1 1] Tank 2 Liquid Level In Real Object
              (`/Game/CoupledTanksProject/Blueprints/TanksRealGraph_Widget.AddActualHeightTank2` _astanks_real_graph_widget (`/Game/CoupledTanksProject/Blueprints/BP_TanksUdpRecv.Tank2ReceivedValue` (`self.TanksUDPRecv`))))
            (:`then_2`
              ;[1 1 1] Tank 3 Liquid Level In Real Object
              (`/Game/CoupledTanksProject/Blueprints/TanksRealGraph_Widget.AddActualHeightTank3` _astanks_real_graph_widget (`/Game/CoupledTanksProject/Blueprints/BP_TanksUdpRecv.Tank3ReceivedValue` (`self.TanksUDPRecv`)))))))
      (:`then_1`
        (bind _returnvalue_2 (`WidgetComponent.GetUserWidgetObject` (`/Game/CoupledTanksProject/Blueprints/TanksMovableWidget_BP.Widget` _output)))
        (if (== (`GameplayStatics.GetObjectClass` _returnvalue_2) "/Game/CoupledTanksProject/BarChart_Widget.BarChart_Widget_C")
          (bind _asbar_chart_widget (cast `/Game/CoupledTanksProject/BarChart_Widget` _returnvalue_2))
          (`/Game/CoupledTanksProject/BarChart_Widget.AddIntegralParameter` _asbar_chart_widget (`/Game/CoupledTanksProject/Blueprints/BP_TanksUdpRecv.ReceivedIntegralParameter` (`self.TanksUDPRecv`))))))))

(fn `UserConstructionScript`)