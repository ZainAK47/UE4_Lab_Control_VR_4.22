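; GameStart is a startup Blueprint that shares a ViveSR reference with the project's levels through a save game.
; On BeginPlay it creates an Experience_SaveGame, stores its ViveSR variable in it and saves it to the ViveSRSlot slot.
; Streaming of the ViveSR sample levels and a quit on framework error are present but disconnected, so neither runs.
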(event `self.ReceiveBeginPlay`
  (`|ExecutionSequence`
    (:`then_0`
      ;[1 1 1] Save ViveSR Reference for all levels to use
      (bind _returnvalue (`GameplayStatics.CreateSaveGameObject` "/Game/CoupledTanksProject/Blueprints/Experience_SaveGame.Experience_SaveGame_C"))
      (set `/Game/CoupledTanksProject/Blueprints/Experience_SaveGame.ViveSR` (`self.ViveSR`) _returnvalue)
      (`GameplayStatics.SaveGameToSlot` _returnvalue "ViveSRSlot"))))

(fn `UserConstructionScript`)