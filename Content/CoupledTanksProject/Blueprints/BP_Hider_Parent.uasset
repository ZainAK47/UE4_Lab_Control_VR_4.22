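; Parent Blueprint for hiders that feed a Plane component's placement into per-tank mask materials in the coupled tanks project.
; Three custom events, one per tank, write the plane's world location and up vector as "pos" and "normal" into that tank's MaskParams Material Parameter Collection.
; Nothing here calls these events, and BeginPlay and Tick are empty.
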(event `self.ReceiveBeginPlay`)

(event `self.ReceiveTick`
  (params (DeltaSeconds :type "Float (single-precision)")))

(event `/Game/CoupledTanksProject/Blueprints/BP_Interface_Hider.Hider1_Function`
  (bind _plane (`self.Plane`))
  (`KismetMaterialLibrary.SetVectorParameterValue` "/Game/CoupledTanksProject/Misc/MaskParams_tank1.MaskParams_tank1" "pos" (`KismetMathLibrary.Conv_VectorToLinearColor` (`SceneComponent.K2_GetComponentLocation` _plane)))
  (`KismetMaterialLibrary.SetVectorParameterValue` "/Game/CoupledTanksProject/Misc/MaskParams_tank1.MaskParams_tank1" "normal" (`KismetMathLibrary.Conv_VectorToLinearColor` (`SceneComponent.GetUpVector` _plane))))

(event `/Game/CoupledTanksProject/Blueprints/BP_Interface_Hider.Hider2_Function`
  (bind _plane (`self.Plane`))
  (`KismetMaterialLibrary.SetVectorParameterValue` "/Game/CoupledTanksProject/Misc/MaskParams_tank2.MaskParams_tank2" "pos" (`KismetMathLibrary.Conv_VectorToLinearColor` (`SceneComponent.K2_GetComponentLocation` _plane)))
  (`KismetMaterialLibrary.SetVectorParameterValue` "/Game/CoupledTanksProject/Misc/MaskParams_tank2.MaskParams_tank2" "normal" (`KismetMathLibrary.Conv_VectorToLinearColor` (`SceneComponent.GetUpVector` _plane))))

(event `/Game/CoupledTanksProject/Blueprints/BP_Interface_Hider.Hider3_Function`
  (bind _plane (`self.Plane`))
  (`KismetMaterialLibrary.SetVectorParameterValue` "/Game/CoupledTanksProject/Misc/MaskParams_tank3.MaskParams_tank3" "pos" (`KismetMathLibrary.Conv_VectorToLinearColor` (`SceneComponent.K2_GetComponentLocation` _plane)))
  (`KismetMaterialLibrary.SetVectorParameterValue` "/Game/CoupledTanksProject/Misc/MaskParams_tank3.MaskParams_tank3" "normal" (`KismetMathLibrary.Conv_VectorToLinearColor` (`SceneComponent.GetUpVector` _plane))))

(fn `UserConstructionScript`)