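; Debug keyboard test actor for the ViveSR pass-through camera and depth framework, with input enabled on BeginPlay.
; Keys start or stop the framework, switch virtual/mixed display, add a Plane depth material, and toggle depth processing, collider updates and collider mesh visibility.
; Another key flips camera brightness between default and maximum.
; Scanning, model and semantic export, and export progress logic exist but are not bound to any event.
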(event `Key|F9`
  (params (Key :type "Key Structure"))
  (:`Pressed`
    (`ViveSR.StartFramework` (`self.ViveSR`))))

(event `Key|F10`
  (params (Key :type "Key Structure"))
  (:`Pressed`
    (`ViveSR.StopFramework` (`self.ViveSR`))))

(event `self.ReceiveBeginPlay`
  (`self.EnableInput` (`GameplayStatics.GetPlayerController` 0)))

(event `Key|Q`
  (params (Key :type "Key Structure"))
  (bind _dualcameraimagerenderer (`ViveSR.DualCameraImageRenderer` (`self.ViveSR`)))
  ;[1 1 1] SetMode
  (:`Pressed`
    (switch `DualCameraDisplayMode` (`ViveSR_DualCameraImageRenderer.dualCameraDisplayMode` _dualcameraimagerenderer)
      (:`VIRTUAL`
        (`ViveSR_DualCameraImageRenderer.SetMode` _dualcameraimagerenderer "MIX"))
      (:`MIX`
        (`ViveSR_DualCameraImageRenderer.SetMode` _dualcameraimagerenderer "VIRTUAL")))))

(event `Key|W`
  (params (Key :type "Key Structure"))
  ;[1 1 1] Add Materials
  (:`Pressed`
    (bind _returnvalue (`PrimitiveComponent.CreateDynamicMaterialInstance` (`self.Plane`) 0 "/SRWorks/Materials/SR_DepthMaterial2.SR_DepthMaterial2" "None"))
    (`KismetArrayLibrary.Array_Add` (`ViveSR_DualCameraImageRenderer.DepthDynamicMaterials` (`ViveSR.DualCameraImageRenderer` (`self.ViveSR`))) _returnvalue)))

(event `Key|A`
  (params (Key :type "Key Structure"))
  ;[1 1 1] Enable/ Disable Depth Process
  (:`Pressed`
    (bind _returnvalue (`SRWorksFunctionLibrary.GetDepthProcessing`))
    (bind _returnvalue_2 (not _returnvalue))
    (bind _returnvalue_3 (`SRWorksFunctionLibrary.EnableDepthProcess` _returnvalue_2))
    (if (== _returnvalue_3 0)
      (`KismetSystemLibrary.PrintString` (`KismetStringLibrary.Concat_StrStr` "Depth Process: " (`KismetStringLibrary.Conv_BoolToString` _returnvalue_2)))
      (else
        (`KismetSystemLibrary.PrintString` (`KismetStringLibrary.Concat_StrStr` "Depth Process: " "false"))))))

(event `Key|S`
  (params (Key :type "Key Structure"))
  (bind _dualcameradepthcollider (`ViveSR.DualCameraDepthCollider` (`self.ViveSR`)))
  (bind _updatedepthcollider (`ViveSR_DualCameraDepthCollider.UpdateDepthCollider` _dualcameradepthcollider))
  ;[1 1 1] Enable/ Disable Depth Collider Process
  (:`Pressed`
    (`ViveSR_DualCameraDepthCollider.SetColliderProcessEnable` _dualcameradepthcollider (not _updatedepthcollider))
    (`KismetSystemLibrary.PrintString` (`KismetStringLibrary.Concat_StrStr` "Depth Collider Process: " (`KismetStringLibrary.Conv_BoolToString` _updatedepthcollider)))))

(event `Key|D`
  (params (Key :type "Key Structure"))
  (bind _dualcameradepthcollider (`ViveSR.DualCameraDepthCollider` (`self.ViveSR`)))
  (bind _collidermeshvisibility (`ViveSR_DualCameraDepthCollider.ColliderMeshVisibility` _dualcameradepthcollider))
  ;[1 1 1] Enable/ Disable Depth Collider Visibility
  (:`Pressed`
    (`ViveSR_DualCameraDepthCollider.SetLiveMeshVisibility` _dualcameradepthcollider (not _collidermeshvisibility))
    (`KismetSystemLibrary.PrintString` (`KismetStringLibrary.Concat_StrStr` "Depth Collider Visibility: " (`KismetStringLibrary.Conv_BoolToString` _collidermeshvisibility)))))

(event `Key|Z`
  (params (Key :type "Key Structure"))
  ;[1 1 1] Start/ Stop Scaning
)

(event `Key|X`
  (params (Key :type "Key Structure"))
  ;[1 1 1] Export Model
)

(event `Key|V`
  (params (Key :type "Key Structure"))
  ;[1 1 1] Export SemanticInfo
)

(event `Key|C`
  (params (Key :type "Key Structure"))
  ;[1 1 1] Get Export Progress
)

(event `Key|E`
  (params (Key :type "Key Structure"))
  (:`Pressed`
    (bind _paraminfo (`SRWorksFunctionLibrary.GetCameraQualityInfo` "BRIGHTNESS"))
    (bind (_status _defaultvalue _min _max _step _defaultmode _value _mode) (break `ParamInfo` _paraminfo))
    (`SRWorksFunctionLibrary.SetCameraQualityInfo` "BRIGHTNESS" (make `ParamInfo` _status _defaultvalue _min _max _step _defaultmode (select `bool` (== _defaultvalue _value) :`false` _defaultvalue :`true` _max) _mode))))

(fn `UserConstructionScript`)